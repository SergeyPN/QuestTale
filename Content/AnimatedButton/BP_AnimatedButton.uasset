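; Trigger-driven actor that plays a flipbook-style animated widget button while the player is in range.
; Two timelines step texture arrays on the widget image: StartEnd plays the intro, then Loop repeats while the player stays.
; Leaving reverses an unfinished intro immediately or an active loop once its cycle ends.
; Presses in range only print a debug string; both speed settings are applied to the StartEnd timeline.
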(event `self.ReceiveBeginPlay`
  (bind _output_get (set `self.InitResult` (and (> (`KismetArrayLibrary.Array_Length` (`self.StartEndFrames`)) 0) (> (`KismetArrayLibrary.Array_Length` (`self.LoopFrames`)) 0))))
  (if _output_get
    (bind _asw_animated_button (cast `/Game/AnimatedButton/W_AnimatedButton` (`WidgetComponent.GetUserWidgetObject` (`self.Widget`))))
    (bind _output_get_2 (set `self.WRef` _asw_animated_button))
    (add `/Game/AnimatedButton/W_AnimatedButton.OnPressedMainButton` _output_get_2 (delegate `OnPressedMainButton_Event_0`))
    (`TimelineComponent.SetPlayRate` (`self.TL_Start/End`) (`self.Start/EndAnimSpeed`))
    (`TimelineComponent.SetPlayRate` (`self.TL_Start/End`) (`self.LoopAnimSpeed`))))

(event `OnPressedMainButton_Event_0`
  (if (`self.InteractSection`)
    (`KismetSystemLibrary.PrintString` "ButtonPressed")))

(event `self.Trigger.OnComponentBeginOverlap`
  (params (OverlappedComponent :type "PrimitiveComponent Object Reference") (OtherActor :type "Actor Object Reference") (OtherComp :type "PrimitiveComponent Object Reference") (OtherBodyIndex :type Integer) (bFromSweep :type Boolean) (SweepResult :type "HitResult Structure (by ref)"))
  (if (`self.InitResult`)
    (if (== OtherActor (`self.PlayerRef`))
      (set `self.InteractSection` true)
      (if (`TimelineComponent.IsReversing` (`self.TL_Start/End`))
        (bind (_direction _alpha) (`Timeline|TL_Start/End` :!label _label)
          (:`Update`
            (`Image.SetBrushFromTexture` (`/Game/AnimatedButton/W_AnimatedButton.IMG_Main` (`self.WRef`)) (`|GetArrayItem` (`self.StartEndFrames`) (`KismetMathLibrary.Round` (`KismetMathLibrary.Lerp` 0.0 (`KismetMathLibrary.Conv_IntToDouble` (`KismetArrayLibrary.Array_LastIndex` (`self.StartEndFrames`))) _alpha))) false))
          (:`Finished`
            (switch `ETimelineDirection` _direction
              (:`Forward`
                (bind (_direction_2 _alpha_2) (`Timeline|TL_Loop` :!label _label_2)
                  (:`Update`
                    (`Image.SetBrushFromTexture` (`/Game/AnimatedButton/W_AnimatedButton.IMG_Main` (`self.WRef`)) (`|GetArrayItem` (`self.LoopFrames`) (`KismetMathLibrary.Round` (`KismetMathLibrary.Lerp` 0.0 (`KismetMathLibrary.Conv_IntToDouble` (`KismetArrayLibrary.Array_LastIndex` (`self.LoopFrames`))) _alpha_2))) false))
                  (:`Finished`
                    (switch `ETimelineDirection` _direction_2
                      (:`Forward`
                        (if (`self.InteractSection`)
                          (goto _label_2 :!via `PlayFromStart`)
                          (else
                            (goto _label :!via `Reverse`)))))))))))
        (elif (`TimelineComponent.IsPlaying` (`self.TL_Start/End`))
          _
          (elif (not (`TimelineComponent.IsPlaying` (`self.TL_Loop`)))
            (goto _label)))))))

(event `self.Trigger.OnComponentEndOverlap`
  (params (OverlappedComponent :type "PrimitiveComponent Object Reference") (OtherActor :type "Actor Object Reference") (OtherComp :type "PrimitiveComponent Object Reference") (OtherBodyIndex :type Integer))
  (if (`self.InitResult`)
    (if (== (`self.PlayerRef`) OtherActor)
      (set `self.InteractSection` false)
      (if (`TimelineComponent.IsPlaying` (`self.TL_Start/End`))
        (goto _label :!via `Reverse`)))))

(fn `UserConstructionScript`)