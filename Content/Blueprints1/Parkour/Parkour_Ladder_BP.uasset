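; Parkour ladder actor that lets the player start climbing up or down through two interaction widgets.
; Each trigger sets a Russian or English label and plays timelines that step the icon through intro and looping frames, reversing on exit.
; InteractwithWidget uses the last animated prompt to send the player's MovePLayer that end's arrow transforms and start state.
; Tick scales and fades both widget buttons by player distance.
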(event `self.ReceiveTick`
  (params (DeltaSeconds :type "Float (single-precision)"))
  (bind _button_817 (`/Game/Assets/tmp/Widget/InteractionWidget.Button_817` (`self.WidgetInteracUP`)))
  (bind (_backgroundcolor_r _backgroundcolor_g _backgroundcolor_b) (break `LinearColor` (`Button.BackgroundColor` _button_817)))
  (bind _returnvalue (`KismetMathLibrary.MapRangeClamped` (`KismetMathLibrary.FClamp` (`KismetMathLibrary.Vector_Distance` (`self.K2_GetActorLocation`) (`self.K2_GetActorLocation` (`self.Player`))) 100.0 500.0) 100.0 500.0 1.0))
  (bind _returnvalue_2 (`KismetMathLibrary.MapRangeClamped` _returnvalue 0.0 1.0 0.5 1.25))
  (`Button.SetBackgroundColor` _button_817 (make `LinearColor` _backgroundcolor_r _backgroundcolor_g _backgroundcolor_b _returnvalue))
  (`Button.SetBackgroundColor` (`/Game/Assets/tmp/Widget/InteractionWidget.Button_817` (`self.WidgetInteracDown`)) (make `LinearColor` _backgroundcolor_r _backgroundcolor_g _backgroundcolor_b _returnvalue))
  (`Widget.SetRenderScale` _button_817 (`KismetMathLibrary.MakeVector2D` _returnvalue_2 _returnvalue_2))
  (`Widget.SetRenderScale` (`/Game/Assets/tmp/Widget/InteractionWidget.Button_817` (`self.WidgetInteracDown`)) (`KismetMathLibrary.MakeVector2D` _returnvalue_2 _returnvalue_2)))

(event `self.ReceiveBeginPlay`
  (`KismetSystemLibrary.Delay` 2.0)
  (bind _outactors (`GameplayStatics.GetAllActorsOfClass` "/Game/Assets/Heroes/Max/MaxCharTest.MaxCharTest_C"))
  (set `self.Player` (`|GetArrayItem` _outactors))
  (bind _asinteraction_widget (cast `/Game/Assets/tmp/Widget/InteractionWidget` (`WidgetComponent.GetUserWidgetObject` (`self.InteractionUP`))))
  (set `self.WidgetInteracUP` _asinteraction_widget)
  (bind _asinteraction_widget_2 (cast `/Game/Assets/tmp/Widget/InteractionWidget` (`WidgetComponent.GetUserWidgetObject` (`self.InteractionDown`))))
  (set `self.WidgetInteracDown` _asinteraction_widget_2)
  (message `/Game/Blueprints1/ToTransfer/BP_interactive.UpdIconWidget` (`self.WidgetInteracUP`) "/Game/Assets/UI/Hint_Circle.Hint_Circle" "" null null null null false null null false "" false)
  (message `/Game/Blueprints1/ToTransfer/BP_interactive.UpdIconWidget` (`self.WidgetInteracDown`) "/Game/Assets/UI/Hint_Circle.Hint_Circle" "" null null null null false null null false "" false))

(event `/Game/Blueprints1/ToTransfer/BP_interactive.InteractWithWidget`
  (switch `int` (`self.NewVar_5`)
    (:`1`
      (set `/Game/Assets/Heroes/Max/MaxCharTest.ParkourState` "NewEnumerator1" (`self.Player`)))
    (:`2`
      (set `/Game/Assets/Heroes/Max/MaxCharTest.ParkourState` "NewEnumerator3" (`self.Player`))))
  (switch `/Game/GameData/ParkourState` (`/Game/Assets/Heroes/Max/MaxCharTest.ParkourState` (`self.Player`))
    (:`NewEnumerator1`
      (set `/Game/Assets/Heroes/Max/MaxCharTest.ParkourState` "NewEnumerator0" (`self.Player`))
      (set `/Game/Assets/Heroes/Max/MaxCharTest.OnParcour` true (`self.Player`))
      (set `self.NewVar_2` false)
      (`self.CloseWidgetUP`)
      (set `self.NewVar_3` (`self.K2_GetActorLocation` (`self.Player`)))
      (`/Game/Assets/Heroes/Max/MaxCharTest.MovePLayer` (`self.Player`) null (`SceneComponent.K2_GetComponentLocation` (`self.ArrowToUp`)) true (`SceneComponent.K2_GetComponentRotation` (`self.ArrowToUp`)) null (`self.StartUpState`) self (`SceneComponent.K2_GetComponentLocation` (`self.ArrowToUPENd`)) null false null null false))
    (:`NewEnumerator3`
      (set `/Game/Assets/Heroes/Max/MaxCharTest.ParkourState` "NewEnumerator0" (`self.Player`))
      (set `/Game/Assets/Heroes/Max/MaxCharTest.OnParcour` true (`self.Player`))
      (set `self.NewVar_2` false)
      (`self.CloseWidgetDown`)
      (`/Game/Assets/Heroes/Max/MaxCharTest.MovePLayer` (`self.Player`) null (`SceneComponent.K2_GetComponentLocation` (`self.ArrowToDown`)) true (`SceneComponent.K2_GetComponentRotation` (`self.ArrowToDown`)) null (`self.StartDownState`) self (`SceneComponent.K2_GetComponentLocation` (`self.ArrowToDownEnd`)) null false null null false))))

(event `CloseWidgetUP`
  (set `self.InteractSection` false :!label _label)
  (if (`TimelineComponent.IsPlaying` (`self.Timeline_1`))
    (bind (_direction _alpha) (`Timeline|Timeline_0` :!via `Reverse` :!label _label_2)
      (:`Update`
        (message `/Game/Blueprints1/ToTransfer/BP_interactive.UpdIconWidget` (`self.WidgetInteracUP`) (`|GetArrayItem` (`self.StartEndFrames`) (`KismetMathLibrary.Round` (`KismetMathLibrary.Lerp` 0.0 (`KismetMathLibrary.Conv_IntToDouble` (`KismetArrayLibrary.Array_LastIndex` (`self.StartEndFrames`))) _alpha))) (`self.IconText`) (`self.StartFlipbook`) (`self.LoopFlipbook`) null null false self null false "" false))
      (:`Finished`
        (set `self.NewVar_5` 1)
        (switch `ETimelineDirection` _direction
          (:`Forward`
            (bind (_direction_2 _alpha_2) (`Timeline|Timeline_1` :!label _label_3)
              (:`Update`
                (if (`self.InteractSection`)
                  (message `/Game/Blueprints1/ToTransfer/BP_interactive.UpdIconWidget` (`self.WidgetInteracUP`) (`|GetArrayItem` (`self.LoopFrames`) (`KismetMathLibrary.Round` (`KismetMathLibrary.Lerp` 0.0 (`KismetMathLibrary.Conv_IntToDouble` (`KismetArrayLibrary.Array_LastIndex` (`self.LoopFrames`))) _alpha_2))) (`self.IconText`) (`self.StartFlipbook`) (`self.LoopFlipbook`) null null false self null false (`self.VisText`) false)
                  (else
                    (`|ExecutionSequence`
                      (:`then_0`
                        (goto _label_3 :!via `Stop`))
                      (:`then_1`
                        (goto _label_2 :!via `Reverse`))))))
              (:`Finished`
                (switch `ETimelineDirection` _direction_2
                  (:`Forward`
                    (if (`self.InteractSection`)
                      (goto _label_3 :!via `PlayFromStart`)
                      (else
                        (goto _label_2 :!via `Reverse`))))))))
          (:`Backward`
            (message `/Game/Blueprints1/ToTransfer/BP_interactive.UpdIconWidget` (`self.WidgetInteracUP`) "/Game/Assets/UI/Hint_Circle.Hint_Circle" "" null null null null false null null false "" false)))))))

(event `self.TriggerToUp.OnComponentBeginOverlap`
  (params (OverlappedComponent :type "PrimitiveComponent Object Reference") (OtherActor :type "Actor Object Reference") (OtherComp :type "PrimitiveComponent Object Reference") (OtherBodyIndex :type Integer) (bFromSweep :type Boolean) (SweepResult :type "HitResult Structure (by ref)"))
  (bind _player (`self.Player`))
  (if (== OtherActor _player)
    (set `/Game/Assets/tmp/Widget/InteractionWidget.Playr_0` _player (`self.WidgetInteracUP`))
    (`self.SetInvUpName`)
    (set `self.InteractSection` true)
    (if (`TimelineComponent.IsReversing` (`self.Timeline_0`))
      (`Widget.SetRenderScale` (`/Game/Assets/tmp/Widget/InteractionWidget.Button_817` (`self.WidgetInteracUP`)) (1.0 1.0) :!label _label_4)
      (goto _label_2)
      (elif (`TimelineComponent.IsPlaying` (`self.Timeline_0`))
        _
        (elif (not (`TimelineComponent.IsPlaying` (`self.Timeline_1`)))
          (goto _label_4))))))

(event `self.TriggerToUp.OnComponentEndOverlap`
  (params (OverlappedComponent :type "PrimitiveComponent Object Reference") (OtherActor :type "Actor Object Reference") (OtherComp :type "PrimitiveComponent Object Reference") (OtherBodyIndex :type Integer))
  (if (== (`self.Player`) OtherActor)
    (goto _label)))

(event `CloseWidgetDown`
  (set `self.InteractSection` false :!label _label_5)
  (if (`TimelineComponent.IsPlaying` (`self.Timeline_1`))
    (bind (_direction _alpha) (`Timeline|Timeline_2` :!via `Reverse` :!label _label_6)
      (:`Update`
        (message `/Game/Blueprints1/ToTransfer/BP_interactive.UpdIconWidget` (`self.WidgetInteracDown`) (`|GetArrayItem` (`self.StartEndFrames`) (`KismetMathLibrary.Round` (`KismetMathLibrary.Lerp` 0.0 (`KismetMathLibrary.Conv_IntToDouble` (`KismetArrayLibrary.Array_LastIndex` (`self.StartEndFrames`))) _alpha))) (`self.IconText`) (`self.StartFlipbook`) (`self.LoopFlipbook`) null null false self null false "" false))
      (:`Finished`
        (set `self.NewVar_5` 2)
        (switch `ETimelineDirection` _direction
          (:`Forward`
            (bind (_direction_2 _alpha_2) (`Timeline|Timeline_3` :!label _label_7)
              (:`Update`
                (if (`self.InteractSection`)
                  (message `/Game/Blueprints1/ToTransfer/BP_interactive.UpdIconWidget` (`self.WidgetInteracDown`) (`|GetArrayItem` (`self.LoopFrames`) (`KismetMathLibrary.Round` (`KismetMathLibrary.Lerp` 0.0 (`KismetMathLibrary.Conv_IntToDouble` (`KismetArrayLibrary.Array_LastIndex` (`self.LoopFrames`))) _alpha_2))) (`self.IconText`) (`self.StartFlipbook`) (`self.LoopFlipbook`) null null false self null false (`self.VisText`) false)
                  (else
                    (`|ExecutionSequence`
                      (:`then_0`
                        (goto _label_7 :!via `Stop`))
                      (:`then_1`
                        (goto _label_6 :!via `Reverse`))))))
              (:`Finished`
                (switch `ETimelineDirection` _direction_2
                  (:`Forward`
                    (if (`self.InteractSection`)
                      (goto _label_7 :!via `PlayFromStart`)
                      (else
                        (goto _label_6 :!via `Reverse`))))))))
          (:`Backward`
            (message `/Game/Blueprints1/ToTransfer/BP_interactive.UpdIconWidget` (`self.WidgetInteracDown`) "/Game/Assets/UI/Hint_Circle.Hint_Circle" "" null null null null false null null false "" false)))))))

(event `self.TriggerToDown.OnComponentBeginOverlap`
  (params (OverlappedComponent :type "PrimitiveComponent Object Reference") (OtherActor :type "Actor Object Reference") (OtherComp :type "PrimitiveComponent Object Reference") (OtherBodyIndex :type Integer) (bFromSweep :type Boolean) (SweepResult :type "HitResult Structure (by ref)"))
  (bind _player (`self.Player`))
  (if (== OtherActor _player)
    (set `/Game/Assets/tmp/Widget/InteractionWidget.Playr_0` _player (`self.WidgetInteracDown`))
    (`self.SetInvDownName`)
    (set `self.InteractSection` true)
    (if (`TimelineComponent.IsReversing` (`self.Timeline_0`))
      (`Widget.SetRenderScale` (`/Game/Assets/tmp/Widget/InteractionWidget.Button_817` (`self.WidgetInteracDown`)) (1.0 1.0) :!label _label_8)
      (goto _label_6)
      (elif (`TimelineComponent.IsPlaying` (`self.Timeline_0`))
        _
        (elif (not (`TimelineComponent.IsPlaying` (`self.Timeline_1`)))
          (goto _label_8))))))

(event `self.TriggerToDown.OnComponentEndOverlap`
  (params (OverlappedComponent :type "PrimitiveComponent Object Reference") (OtherActor :type "Actor Object Reference") (OtherComp :type "PrimitiveComponent Object Reference") (OtherBodyIndex :type Integer))
  (if (== (`self.Player`) OtherActor)
    (goto _label_5)))

(fn `SetInvDownName`
  (switch `/Game/GameData/GameLanguage` (`/Game/Blueprints1/MyGameInstance.Language` (cast `/Game/Blueprints1/MyGameInstance` (`GameplayStatics.GetGameInstance`) :!pure true))
    (:`NewEnumerator0`
      (set `self.VisText` (`self.RusDownName`)))
    (:`NewEnumerator1`
      (set `self.VisText` (`self.EngDownName`)))))

(fn `SetInvUpName`
  (switch `/Game/GameData/GameLanguage` (`/Game/Blueprints1/MyGameInstance.Language` (cast `/Game/Blueprints1/MyGameInstance` (`GameplayStatics.GetGameInstance`) :!pure true))
    (:`NewEnumerator0`
      (set `self.VisText` (`self.RusUpName`)))
    (:`NewEnumerator1`
      (set `self.VisText` (`self.EngUPName`)))))

(fn `UserConstructionScript`)