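; Pickable dirty clothing actor whose MeshIndex selects one of several garment variants.
; The construction script uses that index to set the static mesh, build the inventory item with a matching icon, and assign Russian and English names.
; It then calls SetInvName and positions the Interaction component's height.
; The event graph holds only disabled parent-call stubs.
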(fn `UserConstructionScript`
  (bind _meshindex (`self.MeshIndex`))
  (`StaticMeshComponent.SetStaticMesh` (`self.StaticMesh`) (`|GetArrayItem` (`self.MeshToChoose`) _meshindex))
  (set `self.InventoryItem` (make `/Game/GameData/InventoryItems` "" "NewEnumerator1" (`|GetArrayItem` (`self.IconToChoose`) (`self.MeshIndex`))))
  (switch `int` _meshindex
    (:`0`
      (set `self.RusName` "Шорты")
      (set `self.EngName` "Shorts"))
    (:`1`
      (set `self.RusName` "Майка")
      (set `self.EngName` "Undershirt"))
    (:`2`
      (set `self.RusName` "Штаны")
      (set `self.EngName` "Pants"))
    (:`3`
      (set `self.RusName` "Трусы")
      (set `self.EngName` "Underpants"))
    (:`4`
      (set `self.RusName` "Свитер")
      (set `self.EngName` "Sweater"))
    (:`5`
      (set `self.RusName` "Майка")
      (set `self.EngName` "T-shirt"))
    (:`6`
      (set `self.RusName` "Носки")
      (set `self.EngName` "Socks"))
    (:`7`
      (set `self.RusName` "Носки")
      (set `self.EngName` "Socks"))
    (:`8`
      (set `self.RusName` "Штаны")
      (set `self.EngName` "Pants"))
    (:`9`
      (set `self.RusName` "Майка")
      (set `self.EngName` "T-shirt")))
  (`self.SetInvName`)
  (`SceneComponent.K2_SetRelativeLocation` (`self.Interaction`) (0.0 0.0 50.0) false false))