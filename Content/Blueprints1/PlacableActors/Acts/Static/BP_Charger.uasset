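; BP_Charger is a placeable static actor representing a charger, built on a parent class that supplies its behavior.
; Its construction script positions the inherited-style Interaction and Drop components at fixed relative offsets and sets Russian and English names.
; The event graph adds no logic: BeginPlay and Tick only call the parent, and the overlap event is disabled.
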(event `self.ReceiveBeginPlay`
  (`parent.ReceiveBeginPlay`))

(event `self.ReceiveTick`
  (params (DeltaSeconds :type "Float (single-precision)"))
  (`parent.ReceiveTick` DeltaSeconds))

(fn `UserConstructionScript`
  (`SceneComponent.K2_SetRelativeLocation` (`self.Interaction`) (105.0 -60.0 100.0) false false)
  (`SceneComponent.K2_SetRelativeLocation` (`self.Drop`) (80.0 -40.0 100.0) false false)
  (set `self.RusName` "Зарядка")
  (set `self.EngName` "Charger"))