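; Hidden-object pickup actor that shows an interaction prompt and fires a clicked call when used, if AbleToSee is set.
; Player overlap with its box sets a Russian or English name and runs appear and looping timelines that feed texture frames to the widget, reversing on exit.
; Tick fades and scales the prompt button by player distance.
; ShowInteract and HideInteract toggle the mesh highlight material and a particle effect.
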(event `self.ReceiveTick`
  (params (DeltaSeconds :type "Float (single-precision)"))
  (bind _button_817 (`/Game/Assets/tmp/Widget/InteractionWidget.Button_817` (`self.WidgetInterac`)))
  (bind (_backgroundcolor_r _backgroundcolor_g _backgroundcolor_b) (break `LinearColor` (`Button.BackgroundColor` _button_817)))
  (bind _returnvalue (`KismetMathLibrary.MapRangeClamped` (`KismetMathLibrary.FClamp` (`KismetMathLibrary.Vector_Distance` (`self.K2_GetActorLocation`) (`self.K2_GetActorLocation` (`self.Player`))) 100.0 500.0) 100.0 500.0 1.0))
  (bind _returnvalue_2 (`KismetMathLibrary.MapRangeClamped` _returnvalue 0.0 1.0 0.5 1.25))
  (`Button.SetBackgroundColor` _button_817 (make `LinearColor` _backgroundcolor_r _backgroundcolor_g _backgroundcolor_b _returnvalue))
  (`Widget.SetRenderScale` _button_817 (`KismetMathLibrary.MakeVector2D` _returnvalue_2 _returnvalue_2)))

(event `self.ReceiveBeginPlay`
  (bind _asplayer_controllereee (cast `/Game/Blueprints1/ToTransfer/PlayerControllereee` (`GameplayStatics.GetPlayerController` 0)))
  (add `/Game/Blueprints1/ToTransfer/PlayerControllereee.OnSpawned` _asplayer_controllereee (delegate `CustomEvent_0`))
  (`self.InteractMaterialOff`)
  (message `/Game/Blueprints1/ToTransfer/BP_interactive.UpdIconWidget` (`self.WidgetInterac`) "/Game/Assets/UI/Hint_Circle.Hint_Circle" "" null null null null false null null false "" false))

(event `CustomEvent_0`
  (bind _outactors (`GameplayStatics.GetAllActorsOfClass` "/Game/Assets/tmp/Bp_testr/Player.Player_C"))
  (set `self.Player` (`|GetArrayItem` _outactors))
  (bind _asinteraction_widget (cast `/Game/Assets/tmp/Widget/InteractionWidget` (`WidgetComponent.GetUserWidgetObject` (`self.Interaction`))))
  (bind _output_get (set `self.WidgetInterac` _asinteraction_widget)))

(event `/Game/Blueprints1/ToTransfer/BP_interactive.InteractWithWidget`
  (if (`self.AbleToSee`)
    (`self.HOClicked`)))

(event `ShowInteract`
  (`self.InteractMaterialOn`)
  (`ActorComponent.Activate` (`self.P_DeadMans_Loot`) false))

(event `self.Box.OnComponentBeginOverlap`
  (params (OverlappedComponent :type "PrimitiveComponent Object Reference") (OtherActor :type "Actor Object Reference") (OtherComp :type "PrimitiveComponent Object Reference") (OtherBodyIndex :type Integer) (bFromSweep :type Boolean) (SweepResult :type "HitResult Structure (by ref)"))
  (bind _player (`self.Player`))
  (if (== OtherActor _player)
    (if (`self.AbleToSee`)
      (set `/Game/Assets/tmp/Widget/InteractionWidget.Playr` _player (`self.WidgetInterac`))
      (`self.SetInvName`)
      (set `self.InteractSection` true)
      (if (`TimelineComponent.IsReversing` (`self.St/End`))
        (`GameplayStatics.PlaySound2D` "/Game/Snd_Mus/Snd/ButtonAppear.ButtonAppear" 1.0 1.0 0.0 null null :!label _label)
        (`Widget.SetRenderScale` (`/Game/Assets/tmp/Widget/InteractionWidget.Button_817` (`self.WidgetInterac`)) (1.0 1.0))
        (bind (_direction _alpha) (`Timeline|St/End` :!label _label_2)
          (:`Update`
            (message `/Game/Blueprints1/ToTransfer/BP_interactive.UpdIconWidget` (`self.WidgetInterac`) (`|GetArrayItem` (`self.StartEndFrames`) (`KismetMathLibrary.Round` (`KismetMathLibrary.Lerp` 0.0 (`KismetMathLibrary.Conv_IntToDouble` (`KismetArrayLibrary.Array_LastIndex` (`self.StartEndFrames`))) _alpha))) (`self.IconText`) (`self.StartFlipbook`) (`self.LoopFlipbook`) null null false self null false "" false))
          (:`Finished`
            (switch `ETimelineDirection` _direction
              (:`Forward`
                (bind (_direction_2 _alpha_2) (`Timeline|Looping` :!label _label_3)
                  (:`Update`
                    (if (`self.InteractSection`)
                      (message `/Game/Blueprints1/ToTransfer/BP_interactive.UpdIconWidget` (`self.WidgetInterac`) (`|GetArrayItem` (`self.LoopFrames`) (`KismetMathLibrary.Round` (`KismetMathLibrary.Lerp` 0.0 (`KismetMathLibrary.Conv_IntToDouble` (`KismetArrayLibrary.Array_LastIndex` (`self.LoopFrames`))) _alpha_2))) (`self.IconText`) (`self.StartFlipbook`) (`self.LoopFlipbook`) null null false self null false (`self.VisText`) false)
                      (else
                        (`|ExecutionSequence`
                          (:`then_0`
                            (goto _label_3 :!via `Stop`))
                          (:`then_1`
                            (`GameplayStatics.PlaySound2D` "/Game/Snd_Mus/Snd/ButtonDisappear.ButtonDisappear" 1.0 1.0 0.0 null null :!label _label_4)
                            (goto _label_2 :!via `Reverse`))))))
                  (:`Finished`
                    (switch `ETimelineDirection` _direction_2
                      (:`Forward`
                        (if (`self.InteractSection`)
                          (goto _label_3 :!via `PlayFromStart`)))))))
              (:`Backward`
                (message `/Game/Blueprints1/ToTransfer/BP_interactive.UpdIconWidget` (`self.WidgetInterac`) "/Game/Assets/UI/Hint_Circle.Hint_Circle" "" null null null null false null null false "" false)))))
        (elif (`TimelineComponent.IsPlaying` (`self.St/End`))
          _
          (elif (not (`TimelineComponent.IsPlaying` (`self.Looping`)))
            (goto _label)))))))

(event `HideInteract`
  (`ActorComponent.Deactivate` (`self.P_DeadMans_Loot`))
  (`self.InteractMaterialOff`)
  (set `self.InteractSection` false :!label _label_5)
  (if (`TimelineComponent.IsPlaying` (`self.Looping`))
    (goto _label_4)))

(event `self.Box.OnComponentEndOverlap`
  (params (OverlappedComponent :type "PrimitiveComponent Object Reference") (OtherActor :type "Actor Object Reference") (OtherComp :type "PrimitiveComponent Object Reference") (OtherBodyIndex :type Integer))
  (if (== (`self.Player`) OtherActor)
    (if (`self.InteractSection`)
      (goto _label_5))))

(fn `InteractMaterialOff`
  (locals (OffMat :type "MaterialInterface Object Reference" :default "MaterialInstanceConstant'/Game/Assets/Materials/MI_HeroBoy.MI_HeroBoy'"))
  (`PrimitiveComponent.SetMaterial` (`self.StaticMesh`) 0 (`local.OffMat`)))

(fn `InteractMaterialOn`
  (locals (OnMat :type "MaterialInterface Object Reference" :default "MaterialInstanceConstant'/Game/Assets/Materials/M_ShineFX_Inst.M_ShineFX_Inst'"))
  (`PrimitiveComponent.SetMaterial` (`self.StaticMesh`) 0 (`local.OnMat`)))

(fn `SetInvName`
  (switch `/Game/GameData/GameLanguage` (`/Game/Blueprints1/MyGameInstance.Language` (cast `/Game/Blueprints1/MyGameInstance` (`GameplayStatics.GetGameInstance`) :!pure true))
    (:`NewEnumerator0`
      (set `self.VisText` (`self.RusName`)))
    (:`NewEnumerator1`
      (set `self.VisText` (`self.EngName`)))))

(fn `UserConstructionScript`
  (`SceneComponent.K2_SetRelativeLocation` (`self.Interaction`) (`KismetMathLibrary.MakeVector` 0.0 0.0 (.z (`self.GetActorBounds` false))) false false))

(fn `View`
  (params (Selection :type "/Game/Assets/tmp/Widget/StateWidget Enum" :default "NewEnumerator0"))
  (bind _widgetinterac (`self.WidgetInterac`))
  (switch `/Game/Assets/tmp/Widget/StateWidget` Selection
    (:`NewEnumerator0`
      (`/Game/Assets/tmp/Widget/InteractionWidget.Show UP?` _widgetinterac "NewEnumerator0" null))
    (:`NewEnumerator1`
      (set `self.Switcher` 0)
      (`/Game/Assets/tmp/Widget/InteractionWidget.Show UP?` _widgetinterac "NewEnumerator1" null))
    (:`NewEnumerator2`
      (`/Game/Assets/tmp/Widget/InteractionWidget.Show UP?` _widgetinterac "NewEnumerator2" null))))