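; BP_doors is an interactable door that shows an animated, localized prompt and can move the player between rooms.
; Box overlap drives two timelines that feed intro/outro and looping frames to its InteractionWidget, with the name in Russian or English.
; On interaction, a room index either fires the DoorClicked dispatcher, as unusable doors do, or switches camera and, after a delay, teleports the player to that room's door actor.
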(event `self.ReceiveBeginPlay`
  (bind _asplayer_controllereee (cast `/Game/Assets/tmp/Bp_testr/PlayerControllereee` (`GameplayStatics.GetPlayerController` 0)))
  (add `/Game/Assets/tmp/Bp_testr/PlayerControllereee.OnSpawned` _asplayer_controllereee (delegate `CustomEvent_0`))
  (bind _asinteraction_widget (cast `/Game/Assets/tmp/Widget/InteractionWidget` (`WidgetComponent.GetUserWidgetObject` (`self.Interaction`))))
  (bind _output_get (set `self.WidgetInterac` _asinteraction_widget)))

(event `CustomEvent_0`
  (bind _outactors (`GameplayStatics.GetAllActorsOfClass` "/Game/Assets/tmp/Bp_testr/Player.Player_C"))
  (set `self.Player` (`|GetArrayItem` _outactors)))

(event `/Game/Assets/tmp/Bp_testr/BP_interactive.InteractWithWidget`
  (bind _player (`self.Player`))
  (bind _player_2 (`self.Player`))
  (`KismetSystemLibrary.PrintString` "че ха ъеогя")
  (if (not (`/Game/Assets/tmp/Bp_testr/Player.ChangeLock` _player_2))
    (set `/Game/Assets/tmp/Bp_testr/Player.ChangeLock` true _player_2)
    (if (`self.AbleToUse`)
      (switch `int` (`self.NewVar_0`)
        (:`0`
          (`KismetSystemLibrary.PrintString` "qqqqweee" :!label _label)
          (`self.DoorClicked` self)
          (set `/Game/Assets/tmp/Bp_testr/Player.ChangeLock` false _player_2))
        (:`1`
          (`NavMovementComponent.StopActiveMovement` (`Character.CharacterMovement` (`self.Player`)))
          (set `/Game/Assets/tmp/Bp_testr/Player.ChangeLock` false _player_2)
          (`/Game/Assets/tmp/Bp_testr/PlayerControllereee.SetCamera` (cast `/Game/Assets/tmp/Bp_testr/PlayerControllereee` (`GameplayStatics.GetPlayerController` 0) :!pure true) (`self.NewVar_0`))
          (`KismetSystemLibrary.Delay` 0.5)
          (bind _returnvalue (`GameplayStatics.GetActorOfClass` "/Game/Blueprints/PlacableActors/Doors/BP_doors_MainRoom1.BP_doors_MainRoom1_C"))
          (bind (_returnvalue_x _returnvalue_y) (`KismetMathLibrary.BreakVector` (`self.K2_GetActorLocation` _returnvalue)))
          (`self.K2_SetActorLocation` _player (`KismetMathLibrary.MakeVector` _returnvalue_x _returnvalue_y 100.0) false false)
          (`self.K2_SetActorRotation` _player (struct :`Yaw` 200.0) false))
        (:`2`
          (`NavMovementComponent.StopActiveMovement` (`Character.CharacterMovement` (`self.Player`)))
          (set `/Game/Assets/tmp/Bp_testr/Player.ChangeLock` false _player_2)
          (`/Game/Assets/tmp/Bp_testr/PlayerControllereee.SetCamera` (cast `/Game/Assets/tmp/Bp_testr/PlayerControllereee` (`GameplayStatics.GetPlayerController` 0) :!pure true) (`self.NewVar_0`))
          (`KismetSystemLibrary.Delay` 0.5)
          (bind _returnvalue_2 (`GameplayStatics.GetActorOfClass` "/Game/Blueprints/PlacableActors/Doors/BP_doors_MainRoom2.BP_doors_MainRoom2_C"))
          (bind (_returnvalue_x_2 _returnvalue_y_2) (`KismetMathLibrary.BreakVector` (`self.K2_GetActorLocation` _returnvalue_2)))
          (`self.K2_SetActorLocation` _player (`KismetMathLibrary.MakeVector` _returnvalue_x_2 _returnvalue_y_2 100.0) false false))
        (:`3`
          (`NavMovementComponent.StopActiveMovement` (`Character.CharacterMovement` _player))
          (set `/Game/Assets/tmp/Bp_testr/Player.ChangeLock` false _player_2)
          (`/Game/Assets/tmp/Bp_testr/PlayerControllereee.SetCamera` (cast `/Game/Assets/tmp/Bp_testr/PlayerControllereee` (`GameplayStatics.GetPlayerController` 0) :!pure true) (`self.NewVar_0`))
          (`KismetSystemLibrary.Delay` 0.5)
          (bind _returnvalue_3 (`GameplayStatics.GetActorOfClass` "/Game/Blueprints/PlacableActors/Doors/BP_doors_Kitchen.BP_doors_Kitchen_C"))
          (bind (_returnvalue_x_3 _returnvalue_y_3) (`KismetMathLibrary.BreakVector` (`self.K2_GetActorLocation` _returnvalue_3)))
          (`self.K2_SetActorLocation` _player (`KismetMathLibrary.MakeVector` _returnvalue_x_3 _returnvalue_y_3 100.0) false false))
        (:`4`
          (`NavMovementComponent.StopActiveMovement` (`Character.CharacterMovement` (`self.Player`)))
          (set `/Game/Assets/tmp/Bp_testr/Player.ChangeLock` false _player_2)
          (`/Game/Assets/tmp/Bp_testr/PlayerControllereee.SetCamera` (cast `/Game/Assets/tmp/Bp_testr/PlayerControllereee` (`GameplayStatics.GetPlayerController` 0) :!pure true) (`self.NewVar_0`))
          (`KismetSystemLibrary.Delay` 0.5)
          (bind _returnvalue_4 (`GameplayStatics.GetActorOfClass` "/Game/Blueprints/PlacableActors/Doors/BP_doors_Bathroom.BP_doors_Bathroom_C"))
          (bind (_returnvalue_x_4 _returnvalue_y_4) (`KismetMathLibrary.BreakVector` (`self.K2_GetActorLocation` _returnvalue_4)))
          (`self.K2_SetActorLocation` _player (`KismetMathLibrary.MakeVector` _returnvalue_x_4 _returnvalue_y_4 100.0) false false)))
      (else
        (goto _label)))))

(event `ExitClecked`
  (set `self.InteractSection` false :!label _label_2)
  (if (`TimelineComponent.IsPlaying` (`self.Looping`))
    (bind (_direction _alpha) (`Timeline|St/End` :!via `Reverse` :!label _label_3)
      (:`Update`
        (message `/Game/Assets/tmp/Bp_testr/BP_interactive.UpdIconWidget` (`self.WidgetInterac`) (`|GetArrayItem` (`self.StartEndFrames`) (`KismetMathLibrary.Round` (`KismetMathLibrary.Lerp` 0.0 (`KismetMathLibrary.Conv_IntToDouble` (`KismetArrayLibrary.Array_LastIndex` (`self.StartEndFrames`))) _alpha))) (`self.IconText`) (`self.StartFlipbook`) (`self.LoopFlipbook`) null null false self null false "" false))
      (:`Finished`
        (switch `ETimelineDirection` _direction
          (:`Forward`
            (bind (_direction_2 _alpha_2) (`Timeline|Looping` :!label _label_4)
              (:`Update`
                (if (`self.InteractSection`)
                  (message `/Game/Assets/tmp/Bp_testr/BP_interactive.UpdIconWidget` (`self.WidgetInterac`) (`|GetArrayItem` (`self.LoopFrames`) (`KismetMathLibrary.Round` (`KismetMathLibrary.Lerp` 0.0 (`KismetMathLibrary.Conv_IntToDouble` (`KismetArrayLibrary.Array_LastIndex` (`self.LoopFrames`))) _alpha_2))) (`self.IconText`) (`self.StartFlipbook`) (`self.LoopFlipbook`) null null false self null false (`self.VisText`) false)
                  (else
                    (`|ExecutionSequence`
                      (:`then_0`
                        (goto _label_4 :!via `Stop`))
                      (:`then_1`
                        (goto _label_3 :!via `Reverse`))))))
              (:`Finished`
                (switch `ETimelineDirection` _direction_2
                  (:`Forward`
                    (if (`self.InteractSection`)
                      (goto _label_4 :!via `PlayFromStart`)
                      (else
                        (goto _label_3 :!via `Reverse`)))))))))))))

(event `self.Box.OnComponentBeginOverlap`
  (params (OverlappedComponent :type "PrimitiveComponent Object Reference") (OtherActor :type "Actor Object Reference") (OtherComp :type "PrimitiveComponent Object Reference") (OtherBodyIndex :type Integer) (bFromSweep :type Boolean) (SweepResult :type "HitResult Structure (by ref)"))
  (bind _player (`self.Player`))
  (if (== OtherActor _player)
    (set `/Game/Assets/tmp/Widget/InteractionWidget.Playr` _player (`self.WidgetInterac`))
    (`self.SetInvName`)
    (set `self.InteractSection` true)
    (if (`TimelineComponent.IsReversing` (`self.St/End`))
      (goto _label_3)
      (elif (`TimelineComponent.IsPlaying` (`self.St/End`))
        _
        (elif (not (`TimelineComponent.IsPlaying` (`self.Looping`)))
          (goto _label_3))))))

(event `self.Box.OnComponentEndOverlap`
  (params (OverlappedComponent :type "PrimitiveComponent Object Reference") (OtherActor :type "Actor Object Reference") (OtherComp :type "PrimitiveComponent Object Reference") (OtherBodyIndex :type Integer))
  (if (== (`self.Player`) OtherActor)
    (goto _label_2)))

(fn `SetInvName`
  (switch `/Game/GameData/GameLanguage` (`/Game/Assets/tmp/Bp_testr/MyGameInstance.Language` (cast `/Game/Assets/tmp/Bp_testr/MyGameInstance` (`GameplayStatics.GetGameInstance`) :!pure true))
    (:`NewEnumerator0`
      (set `self.VisText` (`self.RusName`)))
    (:`NewEnumerator1`
      (set `self.VisText` (`self.EngName`)))))

(fn `UserConstructionScript`)

(fn `View`
  (params (Selection :type "/Game/Assets/tmp/Widget/StateWidget Enum" :default "NewEnumerator0"))
  (bind _widgetinterac (`self.WidgetInterac`))
  (switch `/Game/Assets/tmp/Widget/StateWidget` Selection
    (:`NewEnumerator0`
      (`/Game/Assets/tmp/Widget/InteractionWidget.Show UP?` _widgetinterac "NewEnumerator0" null))
    (:`NewEnumerator1`
      (set `self.Switcher` 0)
      (`/Game/Assets/tmp/Widget/InteractionWidget.Show UP?` _widgetinterac "NewEnumerator1" null))
    (:`NewEnumerator2`
      (`/Game/Assets/tmp/Widget/InteractionWidget.Show UP?` _widgetinterac "NewEnumerator2" null))))