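; BP_PC_Pzzle is a placeable static act actor, apparently a PC puzzle, that supplies animation frames for an interaction icon.
; The construction script calls the parent, then fills the loop and start/end frame arrays with the HO icon set.
; ChangeIconsToComment swaps both arrays to the Comment icon set.
; The event graph holds only disabled stubs, so any playback or puzzle logic lives outside this Blueprint.
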(fn `ChangeIconsToComment`
  (set `self.LoopFrames` (`|MakeArray` "/Game/Assets/UI/Icons/Comment/Looping/CommentIconLoop_01.CommentIconLoop_01" "/Game/Assets/UI/Icons/Comment/Looping/CommentIconLoop_02.CommentIconLoop_02" "/Game/Assets/UI/Icons/Comment/Looping/CommentIconLoop_03.CommentIconLoop_03" "/Game/Assets/UI/Icons/Comment/Looping/CommentIconLoop_04.CommentIconLoop_04" "/Game/Assets/UI/Icons/Comment/Looping/CommentIconLoop_05.CommentIconLoop_05" "/Game/Assets/UI/Icons/Comment/Looping/CommentIconLoop_06.CommentIconLoop_06" :!type "Texture2D Object Reference"))
  (set `self.StartEndFrames` (`|MakeArray` "/Game/Assets/UI/Icons/Comment/Start_End/CommentIconStart_01.CommentIconStart_01" "/Game/Assets/UI/Icons/Comment/Start_End/CommentIconStart_02.CommentIconStart_02" "/Game/Assets/UI/Icons/Comment/Start_End/CommentIconStart_03.CommentIconStart_03" "/Game/Assets/UI/Icons/Comment/Start_End/CommentIconStart_04.CommentIconStart_04" "/Game/Assets/UI/Icons/Comment/Start_End/CommentIconStart_05.CommentIconStart_05" "/Game/Assets/UI/Icons/Comment/Start_End/CommentIconStart_06.CommentIconStart_06" :!type "Texture2D Object Reference")))

(fn `UserConstructionScript`
  (`parent.UserConstructionScript`)
  (set `self.LoopFrames` (`|MakeArray` "/Game/Assets/UI/Icons/Pzzle/Loop/HOIconLoop_01.HOIconLoop_01" "/Game/Assets/UI/Icons/Pzzle/Loop/HOIconLoop_02.HOIconLoop_02" "/Game/Assets/UI/Icons/Pzzle/Loop/HOIconLoop_03.HOIconLoop_03" "/Game/Assets/UI/Icons/Pzzle/Loop/HOIconLoop_04.HOIconLoop_04" "/Game/Assets/UI/Icons/Pzzle/Loop/HOIconLoop_05.HOIconLoop_05" "/Game/Assets/UI/Icons/Pzzle/Loop/HOIconLoop_06.HOIconLoop_06" :!type "Texture2D Object Reference"))
  (set `self.StartEndFrames` (`|MakeArray` "/Game/Assets/UI/Icons/Pzzle/Start_End/HOIconStart_01.HOIconStart_01" "/Game/Assets/UI/Icons/Pzzle/Start_End/HOIconStart_02.HOIconStart_02" "/Game/Assets/UI/Icons/Pzzle/Start_End/HOIconStart_03.HOIconStart_03" "/Game/Assets/UI/Icons/Pzzle/Start_End/HOIconStart_04.HOIconStart_04" "/Game/Assets/UI/Icons/Pzzle/Start_End/HOIconStart_05.HOIconStart_05" "/Game/Assets/UI/Icons/Pzzle/Start_End/HOIconStart_06.HOIconStart_06" :!type "Texture2D Object Reference")))