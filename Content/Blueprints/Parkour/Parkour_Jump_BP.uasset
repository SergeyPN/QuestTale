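; Parkour jump point actor that lets the player move up or down between two arrow-marked spots.
; Up and down triggers set the player's ParkourState and show a prompt localized in Russian or English, gated by a flag cleared on use.
; Timelines scrub texture arrays to animate each prompt's appear, loop and disappear phases.
; InteractwithWidget closes the prompt and passes the matching arrow's transform and start state to the player's MovePLayer.
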(event `self.ReceiveBeginPlay`
  (`KismetSystemLibrary.Delay` 2.0)
  (bind _outactors (`GameplayStatics.GetAllActorsOfClass` "/Game/Assets/Heroes/Max/MaxCharTest.MaxCharTest_C"))
  (set `self.Player` (`|GetArrayItem` _outactors))
  (bind _asinteraction_widget (cast `/Game/Assets/tmp/Widget/InteractionWidget` (`WidgetComponent.GetUserWidgetObject` (`self.InteractionUP`))))
  (set `self.WidgetInteracUP` _asinteraction_widget)
  (bind _asinteraction_widget_2 (cast `/Game/Assets/tmp/Widget/InteractionWidget` (`WidgetComponent.GetUserWidgetObject` (`self.InteractionDown`))))
  (set `self.WidgetInteracDown` _asinteraction_widget_2))

(event `/Game/Assets/tmp/Bp_testr/BP_interactive.InteractWithWidget`
  (switch `/Game/GameData/ParkourState` (`/Game/Assets/Heroes/Max/MaxCharTest.ParkourState` (`self.Player`))
    (:`NewEnumerator1`
      (set `/Game/Assets/Heroes/Max/MaxCharTest.OnParcour` true (`self.Player`))
      (set `self.NewVar_2` false)
      (`self.CloseWidgetUP`)
      (set `self.NewVar_3` (`self.K2_GetActorLocation` (`self.Player`)))
      (`/Game/Assets/Heroes/Max/MaxCharTest.MovePLayer` (`self.Player`) null (`SceneComponent.K2_GetComponentLocation` (`self.ArrowToUp`)) true (`SceneComponent.K2_GetComponentRotation` (`self.ArrowToUp`)) self (`self.StartUpState`) null (0.0 0.0 0.0) null false null null false))
    (:`NewEnumerator3`
      (set `/Game/Assets/Heroes/Max/MaxCharTest.OnParcour` true (`self.Player`))
      (set `self.NewVar_2` false)
      (`self.CloseWidgetDown`)
      (`/Game/Assets/Heroes/Max/MaxCharTest.MovePLayer` (`self.Player`) null (`SceneComponent.K2_GetComponentLocation` (`self.ArrowToDown`)) true (`SceneComponent.K2_GetComponentRotation` (`self.ArrowToDown`)) self (`self.StartDownState`) null (0.0 0.0 0.0) null false null null false))))

(event `CloseWidgetUP`
  (set `self.InteractSection` false :!label _label)
  (if (`TimelineComponent.IsPlaying` (`self.Timeline_1`))
    (`GameplayStatics.PlaySound2D` "/Game/Snd_Mus/Snd/ButtonDisappear.ButtonDisappear" 1.0 1.0 0.0 null null :!label _label_2)
    (bind (_direction _alpha) (`Timeline|Timeline_0` :!via `Reverse` :!label _label_3)
      (:`Update`
        (message `/Game/Assets/tmp/Bp_testr/BP_interactive.UpdIconWidget` (`self.WidgetInteracUP`) (`|GetArrayItem` (`self.StartEndFrames`) (`KismetMathLibrary.Round` (`KismetMathLibrary.Lerp` 0.0 (`KismetMathLibrary.Conv_IntToDouble` (`KismetArrayLibrary.Array_LastIndex` (`self.StartEndFrames`))) _alpha))) (`self.IconText`) (`self.StartFlipbook`) (`self.LoopFlipbook`) null null false self null false "" false))
      (:`Finished`
        (switch `ETimelineDirection` _direction
          (:`Forward`
            (bind (_direction_2 _alpha_2) (`Timeline|Timeline_1` :!label _label_4)
              (:`Update`
                (if (`self.InteractSection`)
                  (message `/Game/Assets/tmp/Bp_testr/BP_interactive.UpdIconWidget` (`self.WidgetInteracUP`) (`|GetArrayItem` (`self.LoopFrames`) (`KismetMathLibrary.Round` (`KismetMathLibrary.Lerp` 0.0 (`KismetMathLibrary.Conv_IntToDouble` (`KismetArrayLibrary.Array_LastIndex` (`self.LoopFrames`))) _alpha_2))) (`self.IconText`) (`self.StartFlipbook`) (`self.LoopFlipbook`) null null false self null false (`self.VisText`) false)
                  (else
                    (`|ExecutionSequence`
                      (:`then_0`
                        (goto _label_4 :!via `Stop`))
                      (:`then_1`
                        (goto _label_2))))))
              (:`Finished`
                (switch `ETimelineDirection` _direction_2
                  (:`Forward`
                    (if (`self.InteractSection`)
                      (goto _label_4 :!via `PlayFromStart`)
                      (else
                        (goto _label_2)))))))))))))

(event `self.TriggerToUp.OnComponentBeginOverlap`
  (params (OverlappedComponent :type "PrimitiveComponent Object Reference") (OtherActor :type "Actor Object Reference") (OtherComp :type "PrimitiveComponent Object Reference") (OtherBodyIndex :type Integer) (bFromSweep :type Boolean) (SweepResult :type "HitResult Structure (by ref)"))
  (bind _player (`self.Player`))
  (if (== OtherActor _player)
    (if (`self.NewVar_2`)
      (set `/Game/Assets/Heroes/Max/MaxCharTest.ParkourState` "NewEnumerator1" _player)
      (set `/Game/Assets/tmp/Widget/InteractionWidget.Playr_0` _player (`self.WidgetInteracUP`))
      (`self.SetInvUpName`)
      (set `self.InteractSection` true)
      (if (`TimelineComponent.IsReversing` (`self.Timeline_0`))
        (`GameplayStatics.PlaySound2D` "/Game/Snd_Mus/Snd/ButtonAppear.ButtonAppear" 1.0 1.0 0.0 null null :!label _label_5)
        (goto _label_3)
        (elif (`TimelineComponent.IsPlaying` (`self.Timeline_0`))
          _
          (elif (not (`TimelineComponent.IsPlaying` (`self.Timeline_1`)))
            (goto _label_5)))))))

(event `self.TriggerToUp.OnComponentEndOverlap`
  (params (OverlappedComponent :type "PrimitiveComponent Object Reference") (OtherActor :type "Actor Object Reference") (OtherComp :type "PrimitiveComponent Object Reference") (OtherBodyIndex :type Integer))
  (bind _player (`self.Player`))
  (if (== _player OtherActor)
    (set `/Game/Assets/Heroes/Max/MaxCharTest.ParkourState` "NewEnumerator0" _player)
    (goto _label)))

(event `CloseWidgetDown`
  (set `self.InteractSection` false :!label _label_6)
  (if (`TimelineComponent.IsPlaying` (`self.Timeline_1`))
    (`GameplayStatics.PlaySound2D` "/Game/Snd_Mus/Snd/ButtonDisappear.ButtonDisappear" 1.0 1.0 0.0 null null :!label _label_7)
    (bind (_direction _alpha) (`Timeline|Timeline_2` :!via `Reverse` :!label _label_8)
      (:`Update`
        (message `/Game/Assets/tmp/Bp_testr/BP_interactive.UpdIconWidget` (`self.WidgetInteracDown`) (`|GetArrayItem` (`self.StartEndFrames`) (`KismetMathLibrary.Round` (`KismetMathLibrary.Lerp` 0.0 (`KismetMathLibrary.Conv_IntToDouble` (`KismetArrayLibrary.Array_LastIndex` (`self.StartEndFrames`))) _alpha))) (`self.IconText`) (`self.StartFlipbook`) (`self.LoopFlipbook`) null null false self null false "" false))
      (:`Finished`
        (switch `ETimelineDirection` _direction
          (:`Forward`
            (bind (_direction_2 _alpha_2) (`Timeline|Timeline_3` :!label _label_9)
              (:`Update`
                (if (`self.InteractSection`)
                  (message `/Game/Assets/tmp/Bp_testr/BP_interactive.UpdIconWidget` (`self.WidgetInteracDown`) (`|GetArrayItem` (`self.LoopFrames`) (`KismetMathLibrary.Round` (`KismetMathLibrary.Lerp` 0.0 (`KismetMathLibrary.Conv_IntToDouble` (`KismetArrayLibrary.Array_LastIndex` (`self.LoopFrames`))) _alpha_2))) (`self.IconText`) (`self.StartFlipbook`) (`self.LoopFlipbook`) null null false self null false (`self.VisText`) false)
                  (else
                    (`|ExecutionSequence`
                      (:`then_0`
                        (goto _label_9 :!via `Stop`))
                      (:`then_1`
                        (goto _label_7))))))
              (:`Finished`
                (switch `ETimelineDirection` _direction_2
                  (:`Forward`
                    (if (`self.InteractSection`)
                      (goto _label_9 :!via `PlayFromStart`)
                      (else
                        (goto _label_7)))))))))))))

(event `self.TriggerToDown.OnComponentBeginOverlap`
  (params (OverlappedComponent :type "PrimitiveComponent Object Reference") (OtherActor :type "Actor Object Reference") (OtherComp :type "PrimitiveComponent Object Reference") (OtherBodyIndex :type Integer) (bFromSweep :type Boolean) (SweepResult :type "HitResult Structure (by ref)"))
  (bind _player (`self.Player`))
  (if (== OtherActor _player)
    (if (`self.NewVar_2`)
      (set `/Game/Assets/Heroes/Max/MaxCharTest.ParkourState` "NewEnumerator3" _player)
      (set `/Game/Assets/tmp/Widget/InteractionWidget.Playr_0` _player (`self.WidgetInteracDown`))
      (`self.SetInvDownName`)
      (set `self.InteractSection` true)
      (if (`TimelineComponent.IsReversing` (`self.Timeline_0`))
        (`GameplayStatics.PlaySound2D` "/Game/Snd_Mus/Snd/ButtonAppear.ButtonAppear" 1.0 1.0 0.0 null null :!label _label_10)
        (goto _label_8)
        (elif (`TimelineComponent.IsPlaying` (`self.Timeline_0`))
          _
          (elif (not (`TimelineComponent.IsPlaying` (`self.Timeline_1`)))
            (goto _label_10)))))))

(event `self.TriggerToDown.OnComponentEndOverlap`
  (params (OverlappedComponent :type "PrimitiveComponent Object Reference") (OtherActor :type "Actor Object Reference") (OtherComp :type "PrimitiveComponent Object Reference") (OtherBodyIndex :type Integer))
  (bind _player (`self.Player`))
  (if (== _player OtherActor)
    (set `/Game/Assets/Heroes/Max/MaxCharTest.ParkourState` "NewEnumerator0" _player)
    (goto _label_6)))

(fn `SetInvDownName`
  (switch `/Game/GameData/GameLanguage` (`/Game/Assets/tmp/Bp_testr/MyGameInstance.Language` (cast `/Game/Assets/tmp/Bp_testr/MyGameInstance` (`GameplayStatics.GetGameInstance`) :!pure true))
    (:`NewEnumerator0`
      (set `self.VisText` (`self.RusDownName`)))
    (:`NewEnumerator1`
      (set `self.VisText` (`self.EngDownName`)))))

(fn `SetInvUpName`
  (switch `/Game/GameData/GameLanguage` (`/Game/Assets/tmp/Bp_testr/MyGameInstance.Language` (cast `/Game/Assets/tmp/Bp_testr/MyGameInstance` (`GameplayStatics.GetGameInstance`) :!pure true))
    (:`NewEnumerator0`
      (set `self.VisText` (`self.RusUpName`)))
    (:`NewEnumerator1`
      (set `self.VisText` (`self.EngUPName`)))))

(fn `UserConstructionScript`)