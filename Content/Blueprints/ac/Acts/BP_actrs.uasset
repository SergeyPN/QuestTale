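; Interactable pickup actor that shows an animated prompt near the player and, on InteractwithWidget, destroys itself and increments the controller's PizzaCounter.
; It caches the Player and its Interaction widget when the controller fires OnSpawned.
; Box overlaps drive two timelines that index texture arrays as a flipbook icon: StEnd plays intro and reversed outro, Looping repeats while overlapped.
; The construction script sets the widget's relative height from actor bounds.
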(event `self.ReceiveBeginPlay`
  (bind _asplayer_controllereee (cast `/Game/Assets/tmp/Bp_testr/PlayerControllereee` (`GameplayStatics.GetPlayerController` 0)))
  (add `/Game/Assets/tmp/Bp_testr/PlayerControllereee.OnSpawned` _asplayer_controllereee (delegate `CustomEvent_0`)))

(event `CustomEvent_0`
  (bind _outactors (`GameplayStatics.GetAllActorsOfClass` "/Game/Assets/tmp/Bp_testr/Player.Player_C"))
  (set `self.Player` (`|GetArrayItem` _outactors))
  (bind _asinteraction_widget (cast `/Game/Assets/tmp/Widget/InteractionWidget` (`WidgetComponent.GetUserWidgetObject` (`self.Interaction`))))
  (bind _output_get (set `self.WidgetInterac` _asinteraction_widget)))

(event `/Game/Assets/tmp/Bp_testr/BP_interactive.InteractWithWidget`
  (`self.K2_DestroyActor`)
  (bind _asplayer_controllereee (cast `/Game/Assets/tmp/Bp_testr/PlayerControllereee` (`GameplayStatics.GetPlayerController` 0)))
  (`/Engine/EditorBlueprintResources/StandardMacros.IncrementInt` (`/Game/Assets/tmp/Bp_testr/PlayerControllereee.PizzaCounter` _asplayer_controllereee)))

(event `self.ReceiveTick`
  (params (DeltaSeconds :type "Float (single-precision)")))

(event `self.Box.OnComponentBeginOverlap`
  (params (OverlappedComponent :type "PrimitiveComponent Object Reference") (OtherActor :type "Actor Object Reference") (OtherComp :type "PrimitiveComponent Object Reference") (OtherBodyIndex :type Integer) (bFromSweep :type Boolean) (SweepResult :type "HitResult Structure (by ref)"))
  (bind _player (`self.Player`))
  (if (== OtherActor _player)
    (set `/Game/Assets/tmp/Widget/InteractionWidget.Playr` _player (`self.WidgetInterac`))
    (set `self.InteractSection` true)
    (if (`TimelineComponent.IsReversing` (`self.St/End`))
      (bind (_direction _alpha) (`Timeline|St/End` :!label _label)
        (:`Update`
          (message `/Game/Assets/tmp/Bp_testr/BP_interactive.UpdIconWidget` (`self.WidgetInterac`) (`|GetArrayItem` (`self.StartEndFrames`) (`KismetMathLibrary.Round` (`KismetMathLibrary.Lerp` 0.0 (`KismetMathLibrary.Conv_IntToDouble` (`KismetArrayLibrary.Array_LastIndex` (`self.StartEndFrames`))) _alpha))) (`self.IconText`) (`self.StartFlipbook`) (`self.LoopFlipbook`) null null false))
        (:`Finished`
          (switch `ETimelineDirection` _direction
            (:`Forward`
              (bind (_direction_2 _alpha_2) (`Timeline|Looping` :!label _label_2)
                (:`Update`
                  (if (`self.InteractSection`)
                    (message `/Game/Assets/tmp/Bp_testr/BP_interactive.UpdIconWidget` (`self.WidgetInterac`) (`|GetArrayItem` (`self.LoopFrames`) (`KismetMathLibrary.Round` (`KismetMathLibrary.Lerp` 0.0 (`KismetMathLibrary.Conv_IntToDouble` (`KismetArrayLibrary.Array_LastIndex` (`self.LoopFrames`))) _alpha_2))) (`self.IconText`) (`self.StartFlipbook`) (`self.LoopFlipbook`) null null false)
                    (else
                      (`|ExecutionSequence`
                        (:`then_0`
                          (goto _label_2 :!via `Stop`))
                        (:`then_1`
                          (goto _label :!via `Reverse`))))))
                (:`Finished`
                  (switch `ETimelineDirection` _direction_2
                    (:`Forward`
                      (if (`self.InteractSection`)
                        (goto _label_2 :!via `PlayFromStart`))))))))))
      (elif (`TimelineComponent.IsPlaying` (`self.St/End`))
        _
        (elif (not (`TimelineComponent.IsPlaying` (`self.Looping`)))
          (goto _label))))))

(event `self.Box.OnComponentEndOverlap`
  (params (OverlappedComponent :type "PrimitiveComponent Object Reference") (OtherActor :type "Actor Object Reference") (OtherComp :type "PrimitiveComponent Object Reference") (OtherBodyIndex :type Integer))
  (if (== (`self.Player`) OtherActor)
    (set `self.InteractSection` false)
    (if (`TimelineComponent.IsPlaying` (`self.Looping`))
      (goto _label :!via `Reverse`))))

(fn `UserConstructionScript`
  (`SceneComponent.K2_SetRelativeLocation` (`self.Interaction`) (`KismetMathLibrary.MakeVector` 0.0 0.0 (.z (`self.GetActorBounds` false))) false false))

(fn `View`
  (params (Selection :type "/Game/Assets/tmp/Widget/StateWidget Enum" :default "NewEnumerator0"))
  (bind _widgetinterac (`self.WidgetInterac`))
  (switch `/Game/Assets/tmp/Widget/StateWidget` Selection
    (:`NewEnumerator0`
      (`/Game/Assets/tmp/Widget/InteractionWidget.Show UP?` _widgetinterac "NewEnumerator0" null))
    (:`NewEnumerator1`
      (set `self.Switcher` 0)
      (`/Game/Assets/tmp/Widget/InteractionWidget.Show UP?` _widgetinterac "NewEnumerator1" null))
    (:`NewEnumerator2`
      (`/Game/Assets/tmp/Widget/InteractionWidget.Show UP?` _widgetinterac "NewEnumerator2" null))))