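; Pickable inventory item that shows an animated interaction prompt when the player enters its box.
; StEnd and Looping timelines step through texture arrays to animate the widget's intro, loop and reversed outro.
; InteractwithWidget fires a clicked call and adds the item to the PlayerController's inventory.
; Only Basket items then lock input, turn the player, count clothes, play the Take montage, hide the mesh and destroy the actor.
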(event `self.ReceiveBeginPlay`
  (bind _outactors (`GameplayStatics.GetAllActorsOfClass` "/Game/Assets/tmp/Bp_testr/Player.Player_C" :!label _label))
  (set `self.Player` (`|GetArrayItem` _outactors))
  (bind _asinteraction_widget (cast `/Game/Assets/tmp/Widget/InteractionWidget` (`WidgetComponent.GetUserWidgetObject` (`self.Interaction`))))
  (bind _output_get (set `self.WidgetInterac` _asinteraction_widget))
  (bind _asplayer_controllereee (cast `/Game/Assets/tmp/Bp_testr/PlayerControllereee` (`GameplayStatics.GetPlayerController` 0)))
  (add `/Game/Assets/tmp/Bp_testr/PlayerControllereee.OnSpawned` _asplayer_controllereee (delegate `CustomEvent_0`)))

(event `CustomEvent_0`
  (goto _label))

(event `/Game/Assets/tmp/Bp_testr/BP_interactive.InteractWithWidget`
  (bind _returnvalue (`GameplayStatics.GetPlayerController` 0))
  (bind _returnvalue_2 (`GameplayStatics.GetPlayerController` 0))
  (bind _player (`self.Player`))
  (bind (_inventoryitem_name _inventoryitem_type) (break `/Game/GameData/InventoryItems` (`self.InventoryItem`)))
  (bind (_returnvalue_roll _returnvalue_pitch _returnvalue_yaw) (`KismetMathLibrary.BreakRotator` (`KismetMathLibrary.FindLookAtRotation` (`self.K2_GetActorLocation` _player) (`self.K2_GetActorLocation`))))
  (if (`self.AbletoUse`)
    (`self.PickableActorClicked` self)
    (bind _asplayer_controllereee (cast `/Game/Assets/tmp/Bp_testr/PlayerControllereee` (`GameplayStatics.GetPlayerController` 0)))
    (`/Game/Assets/tmp/Bp_testr/PlayerControllereee.AddItemToInventory` _asplayer_controllereee self (`self.InventoryItem`))
    (switch `/Game/GameData/ItemsTypes` _inventoryitem_type
      (:`NewEnumerator1`
        (if (`self.NewVar_3`)
          (set `self.NewVar_3` false)
          (`NavMovementComponent.StopActiveMovement` (`Character.CharacterMovement` _player))
          (`self.K2_SetActorRotation` _player (`KismetMathLibrary.MakeRotator` 0.0 0.0 _returnvalue_yaw) false)
          (`self.DisableInput` (`Controller.K2_GetPawn` _returnvalue) _returnvalue)
          (`/Game/Assets/tmp/Bp_testr/PlayerControllereee.Clothes GrabCount` _asplayer_controllereee)
          (`|PlayMontage` (`Character.Mesh` (`self.Player`)) "/Game/Assets/Heroes/Boy/Anims/Montage/Take.Take"
            (:`then`
              (`KismetSystemLibrary.Delay` 0.1)
              (`SceneComponent.SetVisibility` (`self.StaticMesh`) false false)
              (set `self.InteractSection` false :!label _label_2)
              (if (`TimelineComponent.IsPlaying` (`self.Looping`))
                (bind (_direction _alpha) (`Timeline|St/End` :!via `Reverse` :!label _label_3)
                  (:`Update`
                    (message `/Game/Assets/tmp/Bp_testr/BP_interactive.UpdIconWidget` (`self.WidgetInterac`) (`|GetArrayItem` (`self.StartEndFrames`) (`KismetMathLibrary.Round` (`KismetMathLibrary.Lerp` 0.0 (`KismetMathLibrary.Conv_IntToDouble` (`KismetArrayLibrary.Array_LastIndex` (`self.StartEndFrames`))) _alpha))) (`self.IconText`) (`self.StartFlipbook`) (`self.LoopFlipbook`) null null false self null))
                  (:`Finished`
                    (switch `ETimelineDirection` _direction
                      (:`Forward`
                        (bind (_direction_2 _alpha_2) (`Timeline|Looping` :!label _label_4)
                          (:`Update`
                            (if (`self.InteractSection`)
                              (message `/Game/Assets/tmp/Bp_testr/BP_interactive.UpdIconWidget` (`self.WidgetInterac`) (`|GetArrayItem` (`self.LoopFrames`) (`KismetMathLibrary.Round` (`KismetMathLibrary.Lerp` 0.0 (`KismetMathLibrary.Conv_IntToDouble` (`KismetArrayLibrary.Array_LastIndex` (`self.LoopFrames`))) _alpha_2))) (`self.IconText`) (`self.StartFlipbook`) (`self.LoopFlipbook`) null null false self null)
                              (else
                                (`|ExecutionSequence`
                                  (:`then_0`
                                    (goto _label_4 :!via `Stop`))
                                  (:`then_1`
                                    (goto _label_3 :!via `Reverse`))))))
                          (:`Finished`
                            (switch `ETimelineDirection` _direction_2
                              (:`Forward`
                                (if (`self.InteractSection`)
                                  (goto _label_4 :!via `PlayFromStart`))))))))))))
            (:`OnCompleted`
              (`self.EnableInput` (`Controller.K2_GetPawn` _returnvalue_2) _returnvalue_2)
              (`self.K2_DestroyActor`))))))))

(event `self.ReceiveTick`
  (params (DeltaSeconds :type "Float (single-precision)")))

(event `self.Box.OnComponentBeginOverlap`
  (params (OverlappedComponent :type "PrimitiveComponent Object Reference") (OtherActor :type "Actor Object Reference") (OtherComp :type "PrimitiveComponent Object Reference") (OtherBodyIndex :type Integer) (bFromSweep :type Boolean) (SweepResult :type "HitResult Structure (by ref)"))
  (bind _player (`self.Player`))
  (if (== OtherActor _player)
    (if (`self.AbletoUse`)
      (set `/Game/Assets/tmp/Widget/InteractionWidget.Playr` _player (`self.WidgetInterac`))
      (set `self.InteractSection` true)
      (if (`TimelineComponent.IsReversing` (`self.St/End`))
        (goto _label_3)
        (elif (`TimelineComponent.IsPlaying` (`self.St/End`))
          _
          (elif (not (`TimelineComponent.IsPlaying` (`self.Looping`)))
            (goto _label_3)))))))

(event `self.Box.OnComponentEndOverlap`
  (params (OverlappedComponent :type "PrimitiveComponent Object Reference") (OtherActor :type "Actor Object Reference") (OtherComp :type "PrimitiveComponent Object Reference") (OtherBodyIndex :type Integer))
  (if (== (`self.Player`) OtherActor)
    (if (`self.AbletoUse`)
      (goto _label_2))))

(fn `UserConstructionScript`
  (`SceneComponent.K2_SetRelativeLocation` (`self.Interaction`) (`KismetMathLibrary.MakeVector` 0.0 0.0 (.z (`self.GetActorBounds` false))) false false))

(fn `View`
  (params (Selection :type "/Game/Assets/tmp/Widget/StateWidget Enum" :default "NewEnumerator0"))
  (bind _widgetinterac (`self.WidgetInterac`))
  (switch `/Game/Assets/tmp/Widget/StateWidget` Selection
    (:`NewEnumerator0`
      (`/Game/Assets/tmp/Widget/InteractionWidget.Show UP?` _widgetinterac "NewEnumerator0" null))
    (:`NewEnumerator1`
      (set `self.Switcher` 0)
      (`/Game/Assets/tmp/Widget/InteractionWidget.Show UP?` _widgetinterac "NewEnumerator1" null))
    (:`NewEnumerator2`
      (`/Game/Assets/tmp/Widget/InteractionWidget.Show UP?` _widgetinterac "NewEnumerator2" null))))