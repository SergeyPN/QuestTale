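; A pickable inventory actor for dirty clothes that can take one of several mesh variants.
; Its construction script uses MeshIndex to set the static mesh and build the InventoryItem struct from the mesh's display name, a fixed enum value and the matching icon.
; It then runs the parent construction script.
; The event graph holds only disabled placeholder events, so the Blueprint adds no runtime logic of its own.
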(fn `UserConstructionScript`
  (bind _output (`|GetArrayItem` (`self.MeshToChoose`) (`self.MeshIndex`)))
  (`StaticMeshComponent.SetStaticMesh` (`self.StaticMesh`) _output)
  (set `self.InventoryItem` (make `/Game/GameData/InventoryItems` (`KismetSystemLibrary.GetDisplayName` _output) "NewEnumerator1" (`|GetArrayItem` (`self.IconToChoose`) (`self.MeshIndex`))))
  (`parent.UserConstructionScript`))