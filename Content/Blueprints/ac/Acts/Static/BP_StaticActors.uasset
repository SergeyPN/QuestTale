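; Static interactable actor that shows an animated icon prompt when the player enters its box and, if droppable, a drop widget on interaction.
; StEnd and Looping timelines scrub texture arrays as flipbook intro, loop and reversed outro for the interaction widget.
; Phone and Basket types bind to player controller events that hide the drop widget and restore the prompt.
; The construction script sets both widget heights from actor bounds.
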(event `self.ReceiveBeginPlay`
  (bind _asplayer_controllereee (cast `/Game/Assets/tmp/Bp_testr/PlayerControllereee` (`GameplayStatics.GetPlayerController` 0)))
  (add `/Game/Assets/tmp/Bp_testr/PlayerControllereee.OnSpawned` _asplayer_controllereee (delegate `CustomEvent_0`)))

(event `CustomEvent_0`
  (bind _outactors (`GameplayStatics.GetAllActorsOfClass` "/Game/Assets/tmp/Bp_testr/Player.Player_C"))
  (set `self.Player` (`|GetArrayItem` _outactors))
  (bind _asinteraction_widget (cast `/Game/Assets/tmp/Widget/InteractionWidget` (`WidgetComponent.GetUserWidgetObject` (`self.Interaction`))))
  (set `self.WidgetInterac` _asinteraction_widget)
  (bind _asw_drop (cast `/Game/Widgets/Inventory/W_Drop` (`WidgetComponent.GetUserWidgetObject` (`self.Drop`))))
  (set `self.Widget Drop` _asw_drop))

(event `/Game/Assets/tmp/Bp_testr/BP_interactive.InteractWithWidget`
  (`self.ActorClicked` self)
  (if (`self.AbleToDrop`)
    (`|ExecutionSequence`
      (:`then_0`
        (set `self.InteractSection` false :!label _label)
        (if (`TimelineComponent.IsPlaying` (`self.Looping`))
          (bind (_direction _alpha) (`Timeline|St/End` :!via `Reverse` :!label _label_2)
            (:`Update`
              (message `/Game/Assets/tmp/Bp_testr/BP_interactive.UpdIconWidget` (`self.WidgetInterac`) (`|GetArrayItem` (`self.StartEndFrames`) (`KismetMathLibrary.Round` (`KismetMathLibrary.Lerp` 0.0 (`KismetMathLibrary.Conv_IntToDouble` (`KismetArrayLibrary.Array_LastIndex` (`self.StartEndFrames`))) _alpha))) (`self.IconText`) (`self.StartFlipbook`) (`self.LoopFlipbook`) null null false self null))
            (:`Finished`
              (switch `ETimelineDirection` _direction
                (:`Forward`
                  (bind (_direction_2 _alpha_2) (`Timeline|Looping` :!label _label_3)
                    (:`Update`
                      (if (`self.InteractSection`)
                        (message `/Game/Assets/tmp/Bp_testr/BP_interactive.UpdIconWidget` (`self.WidgetInterac`) (`|GetArrayItem` (`self.LoopFrames`) (`KismetMathLibrary.Round` (`KismetMathLibrary.Lerp` 0.0 (`KismetMathLibrary.Conv_IntToDouble` (`KismetArrayLibrary.Array_LastIndex` (`self.LoopFrames`))) _alpha_2))) (`self.IconText`) (`self.StartFlipbook`) (`self.LoopFlipbook`) null null false self null)
                        (else
                          (`|ExecutionSequence`
                            (:`then_0`
                              (goto _label_3 :!via `Stop`))
                            (:`then_1`
                              (goto _label_2 :!via `Reverse`))))))
                    (:`Finished`
                      (switch `ETimelineDirection` _direction_2
                        (:`Forward`
                          (if (`self.InteractSection`)
                            (goto _label_3 :!via `PlayFromStart`))))))))))))
      (:`then_2`
        (message `/Game/Assets/tmp/Bp_testr/BP_interactive.UpdIconWidget` (`self.Widget Drop`) (`self.DropWStart`) "" null null null null false null self))
      (:`then_3`
        (switch `/Game/GameData/ItemsTypes` (`self.ActorType`)
          (:`NewEnumerator0`
            (bind _asplayer_controllereee (cast `/Game/Assets/tmp/Bp_testr/PlayerControllereee` (`GameplayStatics.GetPlayerController` 0)))
            (add `/Game/Assets/tmp/Bp_testr/PlayerControllereee.OnPhoneDropped` _asplayer_controllereee (delegate `PhoneDropped`))
            (add `/Game/Widgets/W_Main.DropClosed` (`/Game/Assets/tmp/Bp_testr/PlayerControllereee.W_Menu` _asplayer_controllereee) (delegate `PhoneDropped`)))
          (:`NewEnumerator1`
            (bind _asplayer_controllereee_2 (cast `/Game/Assets/tmp/Bp_testr/PlayerControllereee` (`GameplayStatics.GetPlayerController` 0)))
            (add `/Game/Assets/tmp/Bp_testr/PlayerControllereee.ClothesCollected` _asplayer_controllereee_2 (delegate `CustomEvent`)))))
      (:`then_4`
        (`Widget.SetVisibility` (`self.Widget Drop`) "Visible")))))

(event `self.ReceiveTick`
  (params (DeltaSeconds :type "Float (single-precision)")))

(event `PhoneDropped`
  (`|ExecutionSequence`
    (:`then_0`
      (`Widget.SetVisibility` (`self.Widget Drop`) "Collapsed"))
    (:`then_1`
      (set `self.InteractSection` true :!label _label_4)
      (if (`TimelineComponent.IsReversing` (`self.St/End`))
        (goto _label_2)
        (elif (`TimelineComponent.IsPlaying` (`self.St/End`))
          _
          (elif (not (`TimelineComponent.IsPlaying` (`self.Looping`)))
            (goto _label_2)))))
    (:`then_2`
      (remove `/Game/Assets/tmp/Bp_testr/PlayerControllereee.OnPhoneDropped` (stale `/Game/Assets/tmp/Bp_testr/BP_interactive.InteractWithWidget` _asplayer_controllereee) (delegate `PhoneDropped`))
      (remove `/Game/Assets/tmp/Bp_testr/PlayerControllereee.OnPhoneDropped` (stale `/Game/Assets/tmp/Bp_testr/BP_interactive.InteractWithWidget` _asplayer_controllereee) (delegate `PhoneDropped`)))))

(event `CustomEvent`
  (`|ExecutionSequence`
    (:`then_0`
      (`Widget.SetVisibility` (`self.Widget Drop`) "Collapsed"))
    (:`then_1`
      (goto _label_4))
    (:`then_2`
      (remove `/Game/Assets/tmp/Bp_testr/PlayerControllereee.ClothesCollected` (stale `/Game/Assets/tmp/Bp_testr/BP_interactive.InteractWithWidget` _asplayer_controllereee_2) (delegate `CustomEvent`)))))

(event `self.Box.OnComponentBeginOverlap`
  (params (OverlappedComponent :type "PrimitiveComponent Object Reference") (OtherActor :type "Actor Object Reference") (OtherComp :type "PrimitiveComponent Object Reference") (OtherBodyIndex :type Integer) (bFromSweep :type Boolean) (SweepResult :type "HitResult Structure (by ref)"))
  (bind _player (`self.Player`))
  (if (== OtherActor _player)
    (if (`self.AbleToSee`)
      (set `/Game/Assets/tmp/Widget/InteractionWidget.Playr` _player (`self.WidgetInterac`))
      (goto _label_4))))

(event `self.Box.OnComponentEndOverlap`
  (params (OverlappedComponent :type "PrimitiveComponent Object Reference") (OtherActor :type "Actor Object Reference") (OtherComp :type "PrimitiveComponent Object Reference") (OtherBodyIndex :type Integer))
  (if (== (`self.Player`) OtherActor)
    (if (`self.AbleToSee`)
      (goto _label))))

(fn `UserConstructionScript`
  (bind _origin (`self.GetActorBounds` false))
  (`SceneComponent.K2_SetRelativeLocation` (`self.Interaction`) (`KismetMathLibrary.MakeVector` 0.0 0.0 (.z _origin)) false false)
  (`SceneComponent.K2_SetRelativeLocation` (`self.Drop`) (`KismetMathLibrary.MakeVector` 0.0 0.0 (+ (.z _origin) 10.0)) false false))

(fn `View`
  (params (Selection :type "/Game/Assets/tmp/Widget/StateWidget Enum" :default "NewEnumerator0"))
  (bind _widgetinterac (`self.WidgetInterac`))
  (switch `/Game/Assets/tmp/Widget/StateWidget` Selection
    (:`NewEnumerator0`
      (`/Game/Assets/tmp/Widget/InteractionWidget.Show UP?` _widgetinterac "NewEnumerator0" null))
    (:`NewEnumerator1`
      (set `self.Switcher` 0)
      (`/Game/Assets/tmp/Widget/InteractionWidget.Show UP?` _widgetinterac "NewEnumerator1" null))
    (:`NewEnumerator2`
      (`/Game/Assets/tmp/Widget/InteractionWidget.Show UP?` _widgetinterac "NewEnumerator2" null))))