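; BP_StaticActors_Basket is a basket actor that tracks how many clothes have been collected.
; Its ClothesCount function increments a counter on each call and, when the count reaches ten, casts the first player controller to PlayerControllereee and calls ClothesCollected on it.
; The event graph holds only disabled stub events, so counting relies on ClothesCount being called, and the construction script just runs the parent's.
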(fn `ClothesCount`
  (`/Engine/EditorBlueprintResources/StandardMacros.IncrementInt` (`self.NewVar_3`)
    (:`  `
      (if (== (`self.NewVar_3`) 10)
        (bind _asplayer_controllereee (cast `/Game/Assets/tmp/Bp_testr/PlayerControllereee` (`GameplayStatics.GetPlayerController` 0)))
        (`/Game/Assets/tmp/Bp_testr/PlayerControllereee.ClothesCollected` _asplayer_controllereee)))))

(fn `UserConstructionScript`
  (`parent.UserConstructionScript`))