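; Draggable world object that the player grabs and moves by touch.
; Box overlap shows an animated interaction prompt; interacting toggles between sending the player to the nearest of four side arrows and releasing.
; While the drag widget is held, Tick traces under the finger, clamps the handle's radius, and nudges object and player along it, setting grab axes for that side.
; The construction script fits box and arrows to the assigned mesh.
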(event `111`
  (bind _returnvalue (`GameplayStatics.GetPlayerController` 0))
  (`PrimitiveComponent.SetCollisionResponseToChannel` (`self.StaticMesh`) "ECC_Visibility" "ECR_Block")
  (`self.EnableInput` (`Controller.K2_GetPawn` _returnvalue) _returnvalue))

(event `self.ReceiveTick`
  (params (DeltaSeconds :type "Float (single-precision)"))
  (bind _returnvalue (`self.K2_GetActorLocation`))
  (bind _newvar_2 (`self.NewVar_2`))
  (bind _returnvalue_2 (`KismetMathLibrary.Vector_Distance` _newvar_2 _returnvalue))
  (bind (_returnvalue_x _returnvalue_y) (`KismetMathLibrary.BreakVector` (`KismetMathLibrary.Normal` (- (`SceneComponent.K2_GetComponentLocation` (`self.Dragger1`)) (`self.K2_GetActorLocation`)))))
  (bind _returnvalue_3 (* _returnvalue_y -1.0))
  (if (`/Game/Widgets/DragItems/DragWorldItem_Draggable_W1.Down` (`self.W1(Inn)`))
    (`PrimitiveComponent.SetCollisionResponseToChannel` (`self.StaticMesh`) "ECC_Visibility" "ECR_Ignore")
    (`self.DisableInput` (`Controller.K2_GetPawn` (`GameplayStatics.GetPlayerController` 0)) null)
    (set `self.NewVar_2` (`.Location` (`GameplayStatics.BreakHitResult` (`PlayerController.GetHitResultUnderFingerByChannel` (`GameplayStatics.GetPlayerController` 0) "Touch1" "TraceTypeQuery1" false))))
    (if (!= (`self.NewVar_2`) (0.0 0.0 0.0))
      (`SceneComponent.K2_SetWorldLocation` (`self.Dragger1`) (+ (* (`KismetMathLibrary.GetDirectionUnitVector` _returnvalue _newvar_2) (`KismetMathLibrary.SelectFloat` 150.0 _returnvalue_2 (>= _returnvalue_2 150.0))) _returnvalue) false false)
      (`self.K2_AddActorWorldOffset` (`KismetMathLibrary.MakeVector` _returnvalue_x _returnvalue_y) true)
      (`self.K2_AddActorWorldOffset` (`self.Player`) (`KismetMathLibrary.MakeVector` _returnvalue_x _returnvalue_y) true false)
      (switch `int` (`self.NewVar_3`)
        (:`1`
          (set `/Game/Assets/Heroes/Max/MaxCharTest.ForwardGrab` (* _returnvalue_x -1.0) (`self.Player`))
          (set `/Game/Assets/Heroes/Max/MaxCharTest.RightGrab` _returnvalue_3 (`self.Player`)))
        (:`2`
          (set `/Game/Assets/Heroes/Max/MaxCharTest.ForwardGrab` _returnvalue_x (`self.Player`))
          (set `/Game/Assets/Heroes/Max/MaxCharTest.RightGrab` _returnvalue_y (`self.Player`)))
        (:`3`
          (set `/Game/Assets/Heroes/Max/MaxCharTest.ForwardGrab` _returnvalue_y (`self.Player`))
          (set `/Game/Assets/Heroes/Max/MaxCharTest.RightGrab` _returnvalue_x (`self.Player`)))
        (:`4`
          (set `/Game/Assets/Heroes/Max/MaxCharTest.ForwardGrab` _returnvalue_3 (`self.Player`))
          (set `/Game/Assets/Heroes/Max/MaxCharTest.RightGrab` _returnvalue_x (`self.Player`)))))))

(event `self.ReceiveBeginPlay`
  (`KismetSystemLibrary.Delay` 2.0)
  (bind _outactors (`GameplayStatics.GetAllActorsOfClass` "/Game/Assets/Heroes/Max/MaxCharTest.MaxCharTest_C"))
  (set `self.Player` (`|GetArrayItem` _outactors))
  (bind _asinteraction_widget (cast `/Game/Assets/tmp/Widget/InteractionWidget` (`WidgetComponent.GetUserWidgetObject` (`self.Widget`))))
  (set `self.WidgetInterac` _asinteraction_widget)
  (bind _asdrag_world_item_draggable_w1 (cast `/Game/Widgets/DragItems/DragWorldItem_Draggable_W1` (`WidgetComponent.GetUserWidgetObject` (`self.Dragger1`))))
  (set `self.W1(Inn)` _asdrag_world_item_draggable_w1)
  (set `/Game/Widgets/DragItems/DragWorldItem_Draggable_W1.DragActor` self _asdrag_world_item_draggable_w1)
  (bind _asdrag_world_item_draggable_w (cast `/Game/Widgets/DragItems/DragWorldItem_Draggable_W` (`WidgetComponent.GetUserWidgetObject` (`self.Dragger`))))
  (set `self.W` _asdrag_world_item_draggable_w))

(event `/Game/Assets/tmp/Bp_testr/BP_interactive.InteractWithWidget`
  (bind _player (`self.Player`))
  (`/Engine/EditorBlueprintResources/StandardMacros.FlipFlop`
    (:`A`
      (bind (_arrowtomoveto _newparam) (`self.CheckDistance`))
      (`KismetSystemLibrary.PrintString` (`KismetStringLibrary.Conv_IntToString` _newparam))
      (set `self.NewVar_3` _newparam)
      (set `/Game/Assets/Heroes/Max/MaxCharTest.OnParcour` true _player)
      (`/Game/Assets/Heroes/Max/MaxCharTest.MovePLayer` :`self` _player :`LocToGo` (`SceneComponent.K2_GetComponentLocation` _arrowtomoveto) :`DragArrow` _arrowtomoveto :`DragAction` true :`DragACtor` self))
    (:`B`
      (`/Game/Assets/Heroes/Max/MaxCharTest.StopMovement` (`self.Player`))
      (set `/Game/Assets/Heroes/Max/MaxCharTest.PushItem?` false (`self.Player`))
      (set `/Game/Assets/Heroes/Max/MaxCharTest.OnParcour` false (`self.Player`))
      (set `self.NewVar_1` true))))

(event `DragW_On/Off`
  (if (`|EnumEquality` (`Widget.GetVisibility` (`self.W1(Inn)`)) "Collapsed")
    (`Widget.SetVisibility` (`self.W1(Inn)`) "SelfHitTestInvisible")
    (`Widget.SetVisibility` (`self.W`) "HitTestInvisible")
    (set `/Game/Widgets/DragItems/DragWorldItem_Draggable_W1.IsAbleToDrag?` true (`self.W1(Inn)`))
    (else
      (set `/Game/Widgets/DragItems/DragWorldItem_Draggable_W1.IsAbleToDrag?` false (`self.W1(Inn)`))
      (`Widget.SetVisibility` (`self.W1(Inn)`) "Collapsed")
      (`Widget.SetVisibility` (`self.W`) "Collapsed"))))

(event `self.Box.OnComponentBeginOverlap`
  (params (OverlappedComponent :type "PrimitiveComponent Object Reference") (OtherActor :type "Actor Object Reference") (OtherComp :type "PrimitiveComponent Object Reference") (OtherBodyIndex :type Integer) (bFromSweep :type Boolean) (SweepResult :type "HitResult Structure (by ref)"))
  (bind _player (`self.Player`))
  (if (== OtherActor _player)
    (set `/Game/Assets/tmp/Widget/InteractionWidget.Playr_0` _player (`self.WidgetInterac`))
    (`self.SetInvUpName`)
    (set `self.InteractSection` true)
    (if (`TimelineComponent.IsReversing` (`self.Timeline_0`))
      (bind (_direction _alpha) (`Timeline|Timeline_0` :!label _label)
        (:`Update`
          (message `/Game/Assets/tmp/Bp_testr/BP_interactive.UpdIconWidget` (`self.WidgetInterac`) (`|GetArrayItem` (`self.StartEndFrames`) (`KismetMathLibrary.Round` (`KismetMathLibrary.Lerp` 0.0 (`KismetMathLibrary.Conv_IntToDouble` (`KismetArrayLibrary.Array_LastIndex` (`self.StartEndFrames`))) _alpha))) (`self.IconText`) null null null null false self null false "" false))
        (:`Finished`
          (switch `ETimelineDirection` _direction
            (:`Forward`
              (bind (_direction_2 _alpha_2) (`Timeline|Timeline_1` :!label _label_2)
                (:`Update`
                  (if (`self.InteractSection`)
                    (message `/Game/Assets/tmp/Bp_testr/BP_interactive.UpdIconWidget` (`self.WidgetInterac`) (`|GetArrayItem` (`self.LoopFrames`) (`KismetMathLibrary.Round` (`KismetMathLibrary.Lerp` 0.0 (`KismetMathLibrary.Conv_IntToDouble` (`KismetArrayLibrary.Array_LastIndex` (`self.LoopFrames`))) _alpha_2))) (`self.IconText`) null null null null false self null false (`self.VisText`) false)
                    (else
                      (`|ExecutionSequence`
                        (:`then_0`
                          (goto _label_2 :!via `Stop`))
                        (:`then_1`
                          (goto _label :!via `Reverse`))))))
                (:`Finished`
                  (switch `ETimelineDirection` _direction_2
                    (:`Forward`
                      (if (`self.InteractSection`)
                        (goto _label_2 :!via `PlayFromStart`)
                        (else
                          (goto _label :!via `Reverse`)))))))))))
      (elif (`TimelineComponent.IsPlaying` (`self.Timeline_0`))
        _
        (elif (not (`TimelineComponent.IsPlaying` (`self.Timeline_1`)))
          (goto _label))))))

(event `self.Box.OnComponentEndOverlap`
  (params (OverlappedComponent :type "PrimitiveComponent Object Reference") (OtherActor :type "Actor Object Reference") (OtherComp :type "PrimitiveComponent Object Reference") (OtherBodyIndex :type Integer))
  (if (== (`self.Player`) OtherActor)
    (set `self.InteractSection` false :!label _label_3)
    (if (`TimelineComponent.IsPlaying` (`self.Timeline_1`))
      (goto _label :!via `Reverse`))))

(event `CloseWidgetUP`
  (goto _label_3))

(event `self.Dragger1.OnInputTouchBegin`
  (params (FingerIndex :type "ETouchIndex Enum" :default "Touch1") (TouchedComponent :type "PrimitiveComponent Object Reference")))

(event `self.Dragger1.OnInputTouchEnd`
  (params (FingerIndex :type "ETouchIndex Enum" :default "Touch1") (TouchedComponent :type "PrimitiveComponent Object Reference")))

(fn `22`
  (params (DeltaLocation :type "Vector Structure"))
  (`self.K2_SetActorLocation` (0.0 0.0 0.0)))

(fn `CheckDistance`
  (returns (ArrowToMoveTo :type "ArrowComponent Object Reference") (NewParam :type Integer))
  (locals (Distance :type "Array of Float (double-precision)"))
  (`KismetArrayLibrary.Array_Add` (`local.Distance`) (`KismetMathLibrary.Vector_Distance` (`self.K2_GetActorLocation` (`self.Player`)) (`SceneComponent.K2_GetComponentLocation` (`self.Arrow`))))
  (`KismetArrayLibrary.Array_Add` (`local.Distance`) (`KismetMathLibrary.Vector_Distance` (`self.K2_GetActorLocation` (`self.Player`)) (`SceneComponent.K2_GetComponentLocation` (`self.Arrow1`))))
  (`KismetArrayLibrary.Array_Add` (`local.Distance`) (`KismetMathLibrary.Vector_Distance` (`self.K2_GetActorLocation` (`self.Player`)) (`SceneComponent.K2_GetComponentLocation` (`self.Arrow2`))))
  (`KismetArrayLibrary.Array_Add` (`local.Distance`) (`KismetMathLibrary.Vector_Distance` (`self.K2_GetActorLocation` (`self.Player`)) (`SceneComponent.K2_GetComponentLocation` (`self.Arrow3`))))
  (switch `int` (`KismetMathLibrary.MinOfFloatArray` (`local.Distance`))
    (:`0`
      (return (`self.Arrow`) 1))
    (:`1`
      (return (`self.Arrow1`) 2))
    (:`2`
      (return (`self.Arrow2`) 3))
    (:`3`
      (return (`self.Arrow3`) 4))))

(fn `SetInvUpName`
  (switch `/Game/GameData/GameLanguage` (`/Game/Assets/tmp/Bp_testr/MyGameInstance.Language` (cast `/Game/Assets/tmp/Bp_testr/MyGameInstance` (`GameplayStatics.GetGameInstance`) :!pure true))
    (:`NewEnumerator0`
      (set `self.VisText` (`self.RusUpName`)))
    (:`NewEnumerator1`
      (set `self.VisText` (`self.EngUPName`)))))

(fn `UserConstructionScript`
  (bind _interctboxcollisionsize (`self.InterctBoxCollisionSize`))
  (bind (_min _max) (`StaticMeshComponent.GetLocalBounds` (`self.StaticMesh`)))
  (bind (_returnvalue_x _returnvalue_y) (`KismetMathLibrary.BreakVector` (- _max _min)))
  (bind _returnvalue (* _interctboxcollisionsize _returnvalue_y))
  (bind _returnvalue_2 (* _returnvalue_x _interctboxcollisionsize))
  (`StaticMeshComponent.SetStaticMesh` (`self.StaticMesh`) (`self.MeshToAssign`))
  (`BoxComponent.SetBoxExtent` (`self.Box`) (`KismetMathLibrary.MakeVector` _returnvalue_2 _returnvalue 50.0) true)
  (`SceneComponent.K2_SetRelativeLocation` (`self.Arrow`) (`KismetMathLibrary.MakeVector` _returnvalue_2) false false)
  (`SceneComponent.K2_SetRelativeLocation` (`self.Arrow1`) (`KismetMathLibrary.MakeVector` (* _returnvalue_2 -1.0)) false false)
  (`SceneComponent.K2_SetRelativeLocation` (`self.Arrow2`) (`KismetMathLibrary.MakeVector` 0.0 (* _returnvalue -1.0)) false false)
  (`SceneComponent.K2_SetRelativeLocation` (`self.Arrow3`) (`KismetMathLibrary.MakeVector` 0.0 _returnvalue) false false))