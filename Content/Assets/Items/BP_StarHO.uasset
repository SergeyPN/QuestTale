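; BP_StarHO is a collectible star item that the player picks up by touching it on screen.
; Touching its Box, guarded by a one-time AbleToTouch flag, increments the player controller's Stars, plays a sound, spawns a particle effect and destroys the actor.
; The construction script applies color and roughness through a dynamic material and sizes two nested touch-zone boxes, either square or with separate X and Y extents.
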(event `self.StarHO.OnInputTouchBegin`
  (params (FingerIndex :type "ETouchIndex Enum" :default "Touch1") (TouchedComponent :type "PrimitiveComponent Object Reference")))

(event `self.Box.OnInputTouchBegin`
  (params (FingerIndex :type "ETouchIndex Enum" :default "Touch1") (TouchedComponent :type "PrimitiveComponent Object Reference"))
  (if (`self.AbleToTouch`)
    (set `self.AbleToTouch` false)
    (bind _asplayer_controllereee (cast `/Game/Assets/tmp/Bp_testr/PlayerControllereee` (`GameplayStatics.GetPlayerController` 0)))
    (`/Engine/EditorBlueprintResources/StandardMacros.IncrementInt` (`/Game/Assets/tmp/Bp_testr/PlayerControllereee.Stars` _asplayer_controllereee)
      (:`  `
        (`GameplayStatics.PlaySound2D` "/Game/Snd_Mus/Snd/TakeStar.TakeStar" 1.0 1.0 0.0 null null)
        (`GameplayStatics.SpawnEmitterAtLocation` "/Game/FX/HO/P_HO.P_HO" (`SceneComponent.K2_GetComponentLocation` (`self.StarHO`)))
        (`self.K2_DestroyActor`)))))

(fn `UserConstructionScript`
  (bind _star_touchzone_size (`self.Star_TouchZone_Size`))
  (bind _returnvalue (+ (`self.Star_TouchZone_Size`) 5.0))
  (`|ExecutionSequence`
    (:`then_0`
      (bind _returnvalue_2 (`PrimitiveComponent.CreateDynamicMaterialInstance` (`self.StarHO`) 0 "/Game/Assets/Items/Materials/M_StarHO.M_StarHO" "None"))
      (bind _output_get (set `self.MI_StartHORef` _returnvalue_2))
      (`MaterialInstanceDynamic.SetVectorParameterValue` _output_get "Color" (`self.Color`))
      (`MaterialInstanceDynamic.SetScalarParameterValue` _output_get "RoughStar" (`self.StarRough`)))
    (:`then_1`
      (if (`self.Is_Both_Side_Control?`)
        (`BoxComponent.SetBoxExtent` (`self.Box`) (`KismetMathLibrary.MakeVector` _star_touchzone_size _star_touchzone_size (`self.Star_TouchDepth_Size`)) true)
        (`SceneComponent.K2_SetRelativeLocation` (`self.Box`) (`KismetMathLibrary.MakeVector` 0.0 0.0 (`self.Star_TouchDepth_Size`)) false false)
        (`BoxComponent.SetBoxExtent` (`self.Box1`) (`KismetMathLibrary.MakeVector` _returnvalue _returnvalue (`self.Star_TouchDepth_Size`)) true)
        (`SceneComponent.K2_SetRelativeLocation` (`self.Box1`) (`KismetMathLibrary.MakeVector` 0.0 0.0 (- (`self.Star_TouchDepth_Size`) 0.1)) false false)
        (else
          (`BoxComponent.SetBoxExtent` (`self.Box`) (`KismetMathLibrary.MakeVector` (`self.Star_TouchZone_Size_X`) (`self.Star_TouchZone_Size_Y`) (`self.Star_TouchDepth_Size`)) true)
          (`SceneComponent.K2_SetRelativeLocation` (`self.Box`) (`KismetMathLibrary.MakeVector` 0.0 0.0 (`self.Star_TouchDepth_Size`)) false false)
          (`BoxComponent.SetBoxExtent` (`self.Box1`) (`KismetMathLibrary.MakeVector` (+ (`self.Star_TouchZone_Size_X`) 5.0) (+ (`self.Star_TouchZone_Size_Y`) 5.0) (`self.Star_TouchDepth_Size`)) true)
          (`SceneComponent.K2_SetRelativeLocation` (`self.Box1`) (`KismetMathLibrary.MakeVector` 0.0 0.0 (- (`self.Star_TouchDepth_Size`) 0.5)) false false))))))