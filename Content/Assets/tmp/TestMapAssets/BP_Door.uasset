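; Interactable door that, when open, ends the level by returning to the TestMenu map.
; A sphere overlap shows or hides the player's prompt, while an overlapping Pushable_actor hides the widget.
; Interacting lerps the player onto a Scene component, then plays a montage chosen by StateDoor.
; The open state then swings the mesh on a timeline, sets the camera character's Puzzle flag, blends view to the door and fades out.
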(event `self.ReceiveBeginPlay`
  (bind _ascamera_pc_test (cast `/Game/Assets/tmp/Bp_testr/Camera_PC_test` (`GameplayStatics.GetPlayerCharacter` 0)))
  (set `self.Camera_character` _ascamera_pc_test))

(event `OpenDoor`
  (bind _camera_character (`self.Camera_character`))
  (switch `/Game/Assets/tmp/Bp_testr/Enum` (`self.StateDoor`)
    (:`NewEnumerator0`
      (`/Game/Assets/tmp/Bp_testr/Player.SetMontage` (`self.Charcter`) "/Game/Assets/Heroes/Boy/Anims/Montage/IDK.IDK" null))
    (:`NewEnumerator1`
      (bind _endframe (`/Game/Assets/tmp/Bp_testr/Player.SetMontage` (`self.Charcter`) "/Game/Assets/Heroes/Boy/Anims/Montage/OpenDoor.OpenDoor" null))
      (`KismetSystemLibrary.Delay` _endframe)
      (bind (_direction _alpha) (`Timeline|Timeline_1` :!via `PlayFromStart`)
        (:`Update`
          (`SceneComponent.K2_SetRelativeRotation` (`self.StaticMesh`) (`KismetMathLibrary.MakeRotator` 0.0 0.0 (`KismetMathLibrary.Lerp` 0.0 -110.0 _alpha)) false false))
        (:`Finished`
          (set `/Game/Assets/tmp/Bp_testr/Camera_PC_test.Puzzle` true _camera_character)
          (`PlayerController.SetViewTargetWithBlend` (`GameplayStatics.GetPlayerController` 0) self 1.0 "VTBlend_Linear" 0.0 false)
          (`KismetSystemLibrary.Delay` 0.7)
          (`/Game/Assets/tmp/Widget/ExitWidget.Fade` (`/Game/Assets/tmp/Bp_testr/Camera_PC_test.PlayerWidget` _camera_character))
          (`KismetSystemLibrary.Delay` 0.5)
          (`GameplayStatics.OpenLevel` "TestMenu"))))))

(event `PositionTest`
  (bind _charcter (`self.Charcter`))
  (bind (_direction _alpha) (`Timeline|Timeline_0` :!via `PlayFromStart`)
    (:`Update`
      (`self.K2_SetActorLocationAndRotation` _charcter (`KismetMathLibrary.VLerp` (`self.K2_GetActorLocation` _charcter) (`SceneComponent.K2_GetComponentLocation` (`self.Scene`)) _alpha) (`KismetMathLibrary.RLerp` (`self.K2_GetActorRotation` (`self.Charcter`)) (`SceneComponent.K2_GetComponentRotation` (`self.Scene`)) _alpha true) false false))
    (:`Finished`
      (`self.OpenDoor`))))

(event `/Game/Assets/tmp/Bp_testr/BP_interactive.InteractWithWidget`
  (`self.PositionTest`))

(event `self.Sphere.OnComponentBeginOverlap`
  (params (OverlappedComponent :type "PrimitiveComponent Object Reference") (OtherActor :type "Actor Object Reference") (OtherComp :type "PrimitiveComponent Object Reference") (OtherBodyIndex :type Integer) (bFromSweep :type Boolean) (SweepResult :type "HitResult Structure (by ref)"))
  (`|ExecutionSequence`
    (:`then_0`
      (bind _asplayer (cast `/Game/Assets/tmp/Bp_testr/Player` OtherActor))
      (set `self.Charcter` _asplayer)
      (`self.WidgetView` "NewEnumerator0"))
    (:`then_1`
      (cast `/Game/Assets/tmp/Bp_testr/Pushable_actor` OtherActor)
      (`SceneComponent.SetVisibility` (`self.Widget`) false false))))

(event `self.Sphere.OnComponentEndOverlap`
  (params (OverlappedComponent :type "PrimitiveComponent Object Reference") (OtherActor :type "Actor Object Reference") (OtherComp :type "PrimitiveComponent Object Reference") (OtherBodyIndex :type Integer))
  (`|ExecutionSequence`
    (:`then_0`
      (bind _asplayer (cast `/Game/Assets/tmp/Bp_testr/Player` OtherActor))
      (set `self.Charcter` _asplayer)
      (`self.WidgetView` "NewEnumerator1"))
    (:`then_1`
      (cast `/Game/Assets/tmp/Bp_testr/Pushable_actor` OtherActor)
      (`SceneComponent.SetVisibility` (`self.Widget`) true false))))

(fn `UserConstructionScript`)

(fn `WidgetView`
  (params (Selection :type "/Game/Assets/tmp/Widget/StateWidget Enum" :default "NewEnumerator0"))
  (bind _widgetinterac (`self.WidgetInterac`))
  (switch `/Game/Assets/tmp/Widget/StateWidget` Selection
    (:`NewEnumerator0`
      (bind _asinteraction_widget (cast `/Game/Assets/tmp/Widget/InteractionWidget` (`WidgetComponent.GetUserWidgetObject` (`self.Widget`))))
      (bind _output_get (set `self.WidgetInterac` _asinteraction_widget))
      (message `/Game/Assets/tmp/Bp_testr/BP_interactive.UpdIconWidget` _output_get (`self.IconImage`) (`self.IconText`))
      (`/Game/Assets/tmp/Widget/InteractionWidget.ShowUP?` _widgetinterac "NewEnumerator0"))
    (:`NewEnumerator1`
      (`/Engine/EditorBlueprintResources/StandardMacros.IsValid` _widgetinterac
        (:`Is Valid`
          (`/Game/Assets/tmp/Widget/InteractionWidget.ShowUP?` _widgetinterac "NewEnumerator1"))))
    (:`NewEnumerator2`
      (`/Game/Assets/tmp/Widget/InteractionWidget.ShowUP?` _widgetinterac "NewEnumerator2"))))