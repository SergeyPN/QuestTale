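; BP_Bike is an interactable bike actor that shows an interaction prompt and a toggleable description widget.
; Sphere overlap with a Player shows or hides the prompt, updating its icon and text when shown.
; InteractwithWidget alternates a Click state to show or hide the description.
; A looping timer rotates the prompt widget toward the camera of the player character, cached on BeginPlay.
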(event `self.ReceiveBeginPlay`
  (`|ExecutionSequence`
    (:`then_0`
      (bind _ascamera (cast `/Game/Assets/tmp/Bp_testr/Camera` (`GameplayStatics.GetPlayerCharacter` 0)))
      (set `self.Camera` _ascamera))
    (:`then_1`
      (`KismetSystemLibrary.K2_SetTimerDelegate` (delegate `RotationOnActor`) 0.1 true))))

(event `RotationOnActor`
  (bind _interactwidget (`self.InteractWidget`))
  (`self.Camera`
    (:`then`
      (`SceneComponent.K2_SetWorldRotation` _interactwidget (`KismetMathLibrary.FindLookAtRotation` (`SceneComponent.K2_GetComponentLocation` _interactwidget) (`SceneComponent.K2_GetComponentLocation` (`/Game/Assets/tmp/Bp_testr/Camera.Camera` (`self.Camera`)))) false false))
    (:`else`)))

(event `/Game/Assets/tmp/Bp_testr/BP_interactive.InteractWithWidget`
  (switch `int` (`self.Click`)
    (:`0`
      (bind _result (`/Engine/EditorBlueprintResources/StandardMacros.IncrementInt` (`self.Click`))
        (:`  `
          (set `self.Click` _result)
          (`self.ShowDiscription` true))))
    (:`1`
      (set `self.Click` 0)
      (`self.ShowDiscription` false))))

(event `self.Sphere.OnComponentBeginOverlap`
  (params (OverlappedComponent :type "PrimitiveComponent Object Reference") (OtherActor :type "Actor Object Reference") (OtherComp :type "PrimitiveComponent Object Reference") (OtherBodyIndex :type Integer) (bFromSweep :type Boolean) (SweepResult :type "HitResult Structure (by ref)"))
  (cast `/Game/Assets/tmp/Bp_testr/Player` OtherActor)
  (`self.ShowWidget` true))

(event `self.Sphere.OnComponentEndOverlap`
  (params (OverlappedComponent :type "PrimitiveComponent Object Reference") (OtherActor :type "Actor Object Reference") (OtherComp :type "PrimitiveComponent Object Reference") (OtherBodyIndex :type Integer))
  (cast `/Game/Assets/tmp/Bp_testr/Player` OtherActor)
  (`self.ShowWidget` false))

(fn `ShowDiscription`
  (params (Condition :type Boolean))
  (if Condition
    (bind _asdescription_widget (cast `/Game/Assets/tmp/Widget/descriptionWidget` (`WidgetComponent.GetUserWidgetObject` (`self.Widget`))))
    (bind _output_get (set `self.DiscriptionWidget` _asdescription_widget))
    (`/Game/Assets/tmp/Widget/descriptionWidget.ShowUp` _output_get true)
    (else
      (`/Game/Assets/tmp/Widget/descriptionWidget.ShowUp` (`self.DiscriptionWidget`) false))))

(fn `ShowWidget`
  (params (Show :type Boolean))
  (bind _widgetin (`self.WidgetIn`))
  (if Show
    (bind _asinteraction_widget (cast `/Game/Assets/tmp/Widget/InteractionWidget` (`WidgetComponent.GetUserWidgetObject` (`self.InteractWidget`))))
    (bind _output_get (set `self.WidgetIn` _asinteraction_widget))
    (message `/Game/Assets/tmp/Bp_testr/BP_interactive.UpdIconWidget` _output_get (`self.IconImage`) (`self.IconText`))
    (`/Game/Assets/tmp/Widget/InteractionWidget.ShowUP?` _widgetin true)
    (else
      (`/Game/Assets/tmp/Widget/InteractionWidget.ShowUP?` _widgetin false))))

(fn `UserConstructionScript`)