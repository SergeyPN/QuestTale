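; Interactable electrical puzzle actor that shows a world-space prompt while the player overlaps its sphere.
; A looping timer rotates the widget toward the player's camera, and overlap events fill in its icon and text and show or hide it.
; Interacting blends the view to the first Electric actor in the level, sets the character's Puzzle flag and calls Up on the player widget.
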(event `self.ReceiveBeginPlay`
  (`|ExecutionSequence`
    (:`then_0`
      (bind _ascamera (cast `/Game/Assets/tmp/Bp_testr/Camera` (`GameplayStatics.GetPlayerCharacter` 0)))
      (set `self.Camera` _ascamera))
    (:`then_1`
      (`KismetSystemLibrary.K2_SetTimerDelegate` (delegate `RotationOnActor`) 0.1 true))))

(event `RotationOnActor`
  (bind _widget (`self.Widget`))
  (`self.Camera`
    (:`then`
      (`SceneComponent.K2_SetWorldRotation` _widget (`KismetMathLibrary.FindLookAtRotation` (`SceneComponent.K2_GetComponentLocation` _widget) (`SceneComponent.K2_GetComponentLocation` (`/Game/Assets/tmp/Bp_testr/Camera.Camera` (`self.Camera`)))) false false))
    (:`else`)))

(event `/Game/Assets/tmp/Bp_testr/BP_interactive.InteractWithWidget`
  (bind _camera (`self.Camera`))
  (bind _outactors (`GameplayStatics.GetAllActorsOfClass` "/Game/Assets/tmp/Bp_testr/PuzzleTest/Electric.Electric_C"))
  (`PlayerController.SetViewTargetWithBlend` (`GameplayStatics.GetPlayerController` 0) (`|GetArrayItem` _outactors) 0.0 "VTBlend_Linear" 0.0 false)
  (set `/Game/Assets/tmp/Bp_testr/Camera.Puzzle` true _camera)
  (`/Game/Assets/tmp/Widget/ExitWidget.Up` (`/Game/Assets/tmp/Bp_testr/Camera.PlayerWidget` _camera)))

(event `self.Sphere.OnComponentBeginOverlap`
  (params (OverlappedComponent :type "PrimitiveComponent Object Reference") (OtherActor :type "Actor Object Reference") (OtherComp :type "PrimitiveComponent Object Reference") (OtherBodyIndex :type Integer) (bFromSweep :type Boolean) (SweepResult :type "HitResult Structure (by ref)"))
  (cast `/Game/Assets/tmp/Bp_testr/Player` OtherActor)
  (`self.ShowWidget?` true))

(event `self.Sphere.OnComponentEndOverlap`
  (params (OverlappedComponent :type "PrimitiveComponent Object Reference") (OtherActor :type "Actor Object Reference") (OtherComp :type "PrimitiveComponent Object Reference") (OtherBodyIndex :type Integer))
  (cast `/Game/Assets/tmp/Bp_testr/Player` OtherActor)
  (`self.ShowWidget?` false))

(fn `ShowWidget?`
  (params (`Show?` :type Boolean))
  (bind _widgetinterac (`self.WidgetInterac`))
  (if `Show?`
    (bind _asinteraction_widget (cast `/Game/Assets/tmp/Widget/InteractionWidget` (`WidgetComponent.GetUserWidgetObject` (`self.Widget`))))
    (bind _output_get (set `self.WidgetInterac` _asinteraction_widget))
    (message `/Game/Assets/tmp/Bp_testr/BP_interactive.UpdIconWidget` _output_get (`self.IconImage`) (`self.IconText`))
    (`/Game/Assets/tmp/Widget/InteractionWidget.ShowUP?` _widgetinterac true)
    (else
      (`/Game/Assets/tmp/Widget/InteractionWidget.ShowUP?` _widgetinterac false))))

(fn `UserConstructionScript`)