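; Interactable closet that the player breaks open with a required key item, then uses to enter a puzzle view.
; A sphere overlap toggles the prompt widget, and interacting runs a timeline that lerps the player onto a scene point before branching on state.
; When closed, a key check plays either a crowbar chain-break montage and level sequence, or a failure montage.
; When open, the view blends to the first Shkaf actor and shows its items.
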(event `self.ReceiveBeginPlay`
  (bind _ascamera_pc_test (cast `/Game/Assets/tmp/Bp_testr/Camera_PC_test` (`GameplayStatics.GetPlayerCharacter` 0)))
  (set `self.Camera` _ascamera_pc_test))

(event `/Game/Assets/tmp/Bp_testr/BP_interactive.Open?`
  (params (State :type "/Game/Assets/tmp/Widget/StateWidget Enum" :default "NewEnumerator0"))
  (`self.WidgetView` State))

(event `Animation`
  (bind _camera (`self.Camera`))
  (bind _charcter (`self.Charcter`))
  (switch `/Game/Assets/tmp/Bp_testr/Enum` (`self.State`)
    (:`NewEnumerator0`
      (`self.Check`
        (:`true`
          (`/Game/Assets/tmp/Bp_testr/Player.SetMontage` _charcter "/Game/Assets/Heroes/Boy/Anims/Montage/BreakChain.BreakChain" "/Game/Assets/tmp/TestMapAssets/Crowbar.Crowbar")
          (`KismetSystemLibrary.Delay` 1.94)
          (bind (_outactor _returnvalue) (`LevelSequencePlayer.CreateLevelSequencePlayer` (`self.LevelSequenc`) (make `MovieSceneSequencePlaybackSettings` :`bPauseAtEnd` true)))
          (`MovieSceneSequencePlayer.Play` _returnvalue)
          (`KismetSystemLibrary.Delay` (`.SubFrame` (`KismetMathLibrary.BreakQualifiedFrameTime` (`MovieSceneSequencePlayer.GetEndTime` _returnvalue))))
          (`StaticMeshComponent.SetStaticMesh` (`/Game/Assets/tmp/Bp_testr/Player.StaticMesh` (`self.Charcter`)) null)
          (set `self.State` "NewEnumerator1"))
        (:`false`
          (`/Game/Assets/tmp/Bp_testr/Player.SetMontage` _charcter "/Game/Assets/Heroes/Boy/Anims/Montage/IDK.IDK" null))))
    (:`NewEnumerator1`
      (bind _outactors (`GameplayStatics.GetAllActorsOfClass` "/Game/Assets/tmp/Bp_testr/PuzzleTest/Shkaf.Shkaf_C"))
      (bind _output (`|GetArrayItem` _outactors))
      (`PlayerController.SetViewTargetWithBlend` (`GameplayStatics.GetPlayerController` 0) _output 0.0 "VTBlend_Linear" 0.0 false)
      (set `/Game/Assets/tmp/Bp_testr/Camera_PC_test.Puzzle` true _camera)
      (`/Game/Assets/tmp/Bp_testr/PuzzleTest/Shkaf.UpdItems` _output)
      (`/Game/Assets/tmp/Bp_testr/PuzzleTest/Shkaf.ShowUp` _output true)
      (`/Game/Assets/tmp/Widget/ExitWidget.Up` (`/Game/Assets/tmp/Bp_testr/Camera_PC_test.PlayerWidget` _camera) true))))

(event `/Game/Assets/tmp/Bp_testr/BP_interactive.InteractWithWidget`
  (`self.PsitionTest`))

(event `PsitionTest`
  (bind _charcter (`self.Charcter`))
  (bind (_direction _alpha) (`Timeline|Timeline_0` :!via `PlayFromStart`)
    (:`Update`
      (`self.K2_SetActorLocationAndRotation` _charcter (`KismetMathLibrary.VLerp` (`self.K2_GetActorLocation` _charcter) (`SceneComponent.K2_GetComponentLocation` (`self.Scene`)) _alpha) (`KismetMathLibrary.RLerp` (`self.K2_GetActorRotation` (`self.Charcter`)) (`SceneComponent.K2_GetComponentRotation` (`self.Scene`)) _alpha true) false false))
    (:`Finished`
      (`self.Animation`))))

(event `self.Sphere.OnComponentBeginOverlap`
  (params (OverlappedComponent :type "PrimitiveComponent Object Reference") (OtherActor :type "Actor Object Reference") (OtherComp :type "PrimitiveComponent Object Reference") (OtherBodyIndex :type Integer) (bFromSweep :type Boolean) (SweepResult :type "HitResult Structure (by ref)"))
  (bind _asplayer (cast `/Game/Assets/tmp/Bp_testr/Player` OtherActor))
  (set `self.Charcter` _asplayer)
  (`self.WidgetView` "NewEnumerator0"))

(event `self.Sphere.OnComponentEndOverlap`
  (params (OverlappedComponent :type "PrimitiveComponent Object Reference") (OtherActor :type "Actor Object Reference") (OtherComp :type "PrimitiveComponent Object Reference") (OtherBodyIndex :type Integer))
  (bind _asplayer (cast `/Game/Assets/tmp/Bp_testr/Player` OtherActor))
  (set `self.Charcter` _asplayer)
  (`self.WidgetView` "NewEnumerator1"))

(fn `CheckKey`
  (returns (`haveKey?` :type Boolean))
  (for _array_element (`/Game/Assets/tmp/Bp_testr/Player.Key` (`self.Charcter`))
    (return (`KismetTextLibrary.EqualEqual_TextText` _array_element (`self.Needitem`)))))

(fn `UserConstructionScript`)

(fn `WidgetView`
  (params (Condition :type "/Game/Assets/tmp/Widget/StateWidget Enum" :default "NewEnumerator0"))
  (bind _widgetinterac (`self.WidgetInterac`))
  (switch `/Game/Assets/tmp/Widget/StateWidget` Condition
    (:`NewEnumerator0`
      (bind _asinteraction_widget (cast `/Game/Assets/tmp/Widget/InteractionWidget` (`WidgetComponent.GetUserWidgetObject` (`self.Interaction`))))
      (bind _output_get (set `self.WidgetInterac` _asinteraction_widget))
      (message `/Game/Assets/tmp/Bp_testr/BP_interactive.UpdIconWidget` _output_get (`self.IconImage`) (`self.IconText`))
      (`/Game/Assets/tmp/Widget/InteractionWidget.ShowUP?` _widgetinterac "NewEnumerator0"))
    (:`NewEnumerator1`
      (set `self.Switcher` 0)
      (`/Game/Assets/tmp/Widget/InteractionWidget.ShowUP?` _widgetinterac "NewEnumerator1"))
    (:`NewEnumerator2`
      (`/Game/Assets/tmp/Widget/InteractionWidget.ShowUP?` _widgetinterac "NewEnumerator2"))))